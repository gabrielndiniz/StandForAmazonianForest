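; BP_AnimatedShape is a spell component actor that animates from an origin transform to a target transform, then destroys itself.
; SetTransforms starts a timeline whose play rate scales inversely with distance, keeping travel speed consistent.
; Each update lerps the transform, adding a curve-driven height offset and a rotation modifier.
; On finish it snaps to the target, fires OnShapeAnimationCompleted after a short delay, and destroys itself after another.
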(event Custom|StartAnimation
  (Components|Timeline|SetPlayRate (Variables|Default|GetPlayAnimationTimeline) (/ (Variables|Default|GetSpeed) (/ (Math|Vector|Distance(Vector) (.location (Variables|Default|GetOriginTransform)) (.location (Variables|Default|GetTargetTransform))) (Variables|Default|GetSpeedAdjust))))
  (bind (_direction _transformalpha _heightoffset) (Timeline|PlayAnimationTimeline PlayFromStart)
    (:Update
      (Variables|Default|SetLocationModifier (Math|Vector|MakeVector 0.0 0.0 (* (Variables|Default|GetMaxHeight) _heightoffset)))
      (Transformation|SetActorTransform (Math|Transform|MakeTransform (+ (.location (Math|Transform|Lerp(Transform) (Variables|Default|GetOriginTransform) (Variables|Default|GetTargetTransform) _transformalpha)) (Variables|Default|GetLocationModifier)) (Math|Rotator|CombineRotators (.rotation (Math|Transform|Lerp(Transform) (Variables|Default|GetOriginTransform) (Variables|Default|GetTargetTransform) _transformalpha)) (Variables|Default|GetRotatorModifier)) (.scale (Math|Transform|Lerp(Transform) (Variables|Default|GetOriginTransform) (Variables|Default|GetTargetTransform) _transformalpha)))))
    (:Finished
      (Transformation|SetActorTransform (Variables|Default|GetTargetTransform))
      (Utilities|FlowControl|Delay 0.3)
      (Default|CallOnShapeAnimationCompleted self)
      (Utilities|FlowControl|Delay 0.3)
      (Actor|DestroyActor))))

(event EventBeginPlay)

(fn ConstructionScript)

(fn SetTransforms
  (params (OriginTransform :type Transform) (TargetTransform :type Transform))
  (Variables|Default|SetOriginTransform OriginTransform)
  (Variables|Default|SetTargetTransform TargetTransform)
  (CallFunction|StartAnimation))