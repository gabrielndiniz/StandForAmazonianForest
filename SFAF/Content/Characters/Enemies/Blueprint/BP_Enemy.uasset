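; BP_Enemy is a wheeled enemy that visually spins its wheels as it moves.
; On BeginPlay it collects the PhysicsConstraint children of its StaticMesh, each one's first child mesh as a wheel, and a size from that wheel's scaled bounds.
; SpinWheels increments each constraint's relative roll using box and wheel velocity, wheel size and delta time.
; Nothing in these graphs calls SpinWheels, and its while loop returns after one pass.
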(event EventBeginPlay
  (for _array_element (Components|GetChildrenComponents (Variables|Default|GetStaticMesh) false)
    (bind _asphysics_constraint_component (Utilities|Casting|CastToPhysicsConstraintComponent _array_element))
    (Utilities|Array|Add (Variables|Default|GetConstrains) _asphysics_constraint_component)
    (bind _asstatic_mesh_component (Utilities|Casting|CastToStaticMeshComponent (Components|GetChildComponent _asphysics_constraint_component 0)))
    (Utilities|Array|Add (Variables|Default|GetWheels) _asstatic_mesh_component)
    (Utilities|Array|Add (Variables|Default|GetWheelsSize) (* (Math|Vector|DotProduct (.Max (Components|StaticMesh|GetLocalBounds _asstatic_mesh_component)) (Math|Vector|GetUpVector _asstatic_mesh_component)) (Math|Vector|DotProduct (Math|Vector|GetUpVector _asstatic_mesh_component) (Transformation|GetWorldScale _asstatic_mesh_component))))))

(event Collision|EventActorBeginOverlap
  (params (OtherActor :type Actor%20Object%20Reference)))

(event EventTick
  (params (DeltaSeconds :type Float%20%28single-precision%29)))

(fn ConstructionScript
  (|CallParentFunction))

(fn SpinWheels
  (bind _constrains (Variables|Default|GetConstrains))
  (bind _returnvalue (Utilities|Array|LastIndex _constrains))
  (if (Utilities|Array|IsEmpty (Variables|Default|GetConstrains))
    (return)
    (elif (and (== (Utilities|Array|LastIndex (Variables|Default|GetWheels)) _returnvalue) (== _returnvalue (Utilities|Array|LastIndex (Variables|Default|GetWheelsSize))))
      (while (> (Math|Vector|VectorLength (Transformation|GetComponentVelocity (Variables|Default|GetBox))) 0.0)
        (if (Utilities|Operators|EqualEqual :A (Transformation|GetComponentVelocity (Variables|Default|GetBox)) :ErrorTolerance 1e-05)
          (return)
          (else
            (for (_array_element _array_index) (Variables|Default|GetConstrains)
              (Transformation|SetRelativeRotation _array_element (Math|Rotator|MakeRotator (+ (* (Math|Vector|VectorLength (+ (Transformation|GetComponentVelocity (Variables|Default|GetBox)) (Transformation|GetComponentVelocity (Utilities|Array|Get(acopy) (Variables|Default|GetWheels) _array_index)))) (/ (Math|Float|MultiplybyPi (Utilities|Array|Get(acopy) (Variables|Default|GetWheelsSize) _array_index)) 3.6e+02) (Utilities|Time|GetWorldDeltaSeconds)) (.roll (Variables|/Script/Engine.SceneComponent|GetRelativeRotation _array_element))) (.pitch (Variables|/Script/Engine.SceneComponent|GetRelativeRotation _array_element)) (.yaw (Variables|/Script/Engine.SceneComponent|GetRelativeRotation _array_element))) false false))
            (return))))
      (return)
      (else
        (return)))))