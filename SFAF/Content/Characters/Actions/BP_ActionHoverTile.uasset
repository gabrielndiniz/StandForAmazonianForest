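; BP_ActionHoverTile is an action Blueprint that shows a hover plane over the tile given by an index.
; ExecuteAction runs the parent action, moves HoverPlane to the location in the returned data, then returns that data; an index of -1 hides the plane instead.
; SetHoverPlaneLocation skips updates when the requested location nearly matches the current one.
; The plane starts hidden on BeginPlay and needs no Tick.
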(event EventBeginPlay
  (|CallParentFunction)
  (Rendering|SetVisibility (Variables|Default|GetHoverPlane) false false))

(event Collision|EventActorBeginOverlap
  (params (OtherActor :type Actor%20Object%20Reference))
  (|CallParentFunction OtherActor) ; This node is disabled and will not be called.\nDrag off pins to build functionality.
)

(event EventTick
  (params (DeltaSeconds :type Float%20%28single-precision%29))
  (|CallParentFunction DeltaSeconds) ; This node is disabled and will not be called.\nDrag off pins to build functionality.
)

(fn ConstructionScript
  (|CallParentFunction))

(fn SetHoverPlaneLocation
  (params (NewLocation :type Vector) (bHide :type Boolean))
  (bind _hoverplane (Variables|Default|GetHoverPlane))
  (if (Utilities|Operators|NotEqual(!=) NewLocation (Transformation|GetWorldLocation (Variables|Default|GetHoverPlane)) 0.01)
    (if bHide
      (Rendering|SetVisibility _hoverplane false false)
      (else
        (Transformation|SetWorldLocation _hoverplane NewLocation false false)
        (if (not (Rendering|IsVisible (Variables|Default|GetHoverPlane)))
          (Rendering|SetVisibility (Variables|Default|GetHoverPlane) true false))))))

(fn ExecuteAction
  (params (Index :type Integer))
  (bind _tiledata (|CallParentFunction Index))
  (LocalVariables|SetData _tiledata)
  (Utilities|FlowControl|Sequence
    (:then_0
      (if (!= Index -1)
        (CallFunction|SetHoverPlaneLocation (.location (.transform (LocalVariables|GetData))) false)
        (else
          (CallFunction|SetHoverPlaneLocation "0.000000,0.000000,9999.000000" true))))
    (:then_1
      (return (LocalVariables|GetData)))))