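; BP_ActionSelectTileCalculateMinCost is a tile-selection action that shows pathfinding minimum-cost estimates from every grid tile to the selected one.
; On execute it runs the parent action, then loops over all grid positions, computing each minimum cost through the injected FindPathToTarget and registering the tile as discovered with zero start cost.
; It tints its hexagon marker yellow on BeginPlay, and ClearTarget clears reachable instances and moves the marker out of view.
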(event EventBeginPlay
  (|CallParentFunction)
  (Utilities|FlowControl|Delay 0.1)
  (Rendering|Material|SetVectorParameterValueonMaterials (Variables|Default|GetHexagon) "Color" (Math|Conversions|ToVector(LinearColor) (Math|Color|MakeColor 0.8 0.8 0.01))))

(event Collision|EventActorBeginOverlap
  (params (OtherActor :type Actor%20Object%20Reference))
  (|CallParentFunction OtherActor) ; This node is disabled and will not be called.\nDrag off pins to build functionality.
)

(event EventTick
  (params (DeltaSeconds :type Float%20%28single-precision%29))
  (|CallParentFunction DeltaSeconds) ; This node is disabled and will not be called.\nDrag off pins to build functionality.
)

(fn ConstructionScript
  (|CallParentFunction))

(fn ExecuteAction
  (params (Position%201 :type Int%20Point%20Structure) (bHitResult :type Boolean) (Position%202 :type Int%20Point%20Structure))
  (bind (_success _tiledata1 _tiledata2) (|CallParentFunction Position%201 bHitResult Position%202))
  (Utilities|FlowControl|Sequence
    (:then_0
      (Utilities|IsValid (Variables|Default|GetFind%20Path%20to%20Target)
        (:Is%20Valid
          (for _array_element (Default|GetAllGridPositions (Variables|Default|GetGrid))
            (bind _mincost (Default|GetMinimumCostBetweenTwoTiles (Variables|Default|GetFind%20Path%20to%20Target) _array_element Position%201))
            (Default|DiscoverTile (Variables|Default|GetFind%20Path%20to%20Target) (Utilities|Struct|MakeST_PathfindingData _array_element 10 0 _mincost "(X=999,Y=999)"))))))
    (:then_1
      (return _success _tiledata1 _tiledata2))))

(fn SetFindPathtoTarget
  (params (FindPathToTarget :type BP%20Action%20Find%20Path%20to%20Target%20Object%20Reference))
  (Variables|Default|SetFind%20Path%20to%20Target FindPathToTarget))

(fn ClearTarget
  (Components|InstancedStaticMesh|ClearInstances (Variables|Default|GetInstancedStaticMeshReachables))
  (Transformation|SetRelativeLocation (Variables|Default|GetHexagon) "0.000000,0.000000,9999.000000" false false))