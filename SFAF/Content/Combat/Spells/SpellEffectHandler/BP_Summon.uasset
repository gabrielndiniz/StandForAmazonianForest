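; BP_Summon is a spell effect handler that spawns units of a configurable type and team onto the combat grid.
; SpellEffect calls its parent, then finds the BP_ActionAddRemoveUnitFromCombat actor in the world and passes it the summon type and team.
; It loops over the secondary positions and, on each valid tile with no unit, adds a unit with AI off and outside the active list.
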(event EventBeginPlay)

(event Collision|EventActorBeginOverlap
  (params (OtherActor :type Actor%20Object%20Reference)))

(event EventTick
  (params (DeltaSeconds :type Float%20%28single-precision%29)))

(fn ConstructionScript
  (|CallParentFunction))

(fn SpellEffect
  (|CallParentFunction)
  (bind _returnvalue (Actor|GetActorOfClass "/Game/Characters/Actions/Combat/BP_ActionAddRemoveUnitFromCombat.BP_ActionAddRemoveUnitFromCombat_C"))
  (bind _output_get (LocalVariables|SetAddRemoveUnit _returnvalue))
  (Default|SetUnitType _output_get (Variables|Default|GetSummonType))
  (Default|SetTeamNumber (LocalVariables|GetAddRemoveUnit) (Variables|Default|GetSummonTeam))
  (for _array_element (Variables|Default|GetSecondaryPositions)
    (if (.Success (Default|GetTileData (Variables|Default|GetGrid) _array_element))
      (Utilities|IsValid (.UnitOnTyle (Utilities|Struct|BreakST_TileData (.TileData (Default|GetTileData (Variables|Default|GetGrid) _array_element))))
        (:Is%20Not%20Valid
          (Default|SetUseAI (LocalVariables|GetAddRemoveUnit) false)
          (Default|AddUnit (LocalVariables|GetAddRemoveUnit) _array_element false))))))

(fn SetSummonType
  (params (SummonType :type E_UnitType%20Enum :default "NewEnumerator0"))
  (Variables|Default|SetSummonType SummonType))

(fn SetSummonTeam
  (params (SummonTeam :type Byte))
  (Variables|Default|SetSummonTeam SummonTeam))