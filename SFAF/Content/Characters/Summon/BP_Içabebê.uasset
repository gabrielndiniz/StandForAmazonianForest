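; Summoned unit Blueprint for Içabebê that adds visual variation to its static mesh on top of an inherited parent.
; On BeginPlay and on reset, it randomly mirrors the enlarged mesh on X and Y through negative scale and slightly varies its height.
; When the parent's delayed hide-unit event fires, it scales the mesh to zero.
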(event EventBeginPlay
  (|CallParentFunction)
  (Transformation|SetRelativeScale3D (Variables|Default|GetStaticMesh) (Math|Vector|MakeVector (* (Math|Conversions|ToFloat(Integer) (- (* (Math|Conversions|ToInteger(Boolean) (Math|Random|RandomBool)) 2) 1)) 4.0) (* (Math|Conversions|ToFloat(Integer) (- (* (Math|Conversions|ToInteger(Boolean) (Math|Random|RandomBool)) 2) 1)) 4.0) (* (Math|Random|RandomFloatinRange 0.8 1.2) 4.0))))

(event EventOnReset
  (|CallParentFunction)
  (Transformation|SetRelativeScale3D (Variables|Default|GetStaticMesh) (Math|Vector|MakeVector (* (Math|Conversions|ToFloat(Integer) (- (* (Math|Conversions|ToInteger(Boolean) (Math|Random|RandomBool)) 2) 1)) 4.0) (* (Math|Conversions|ToFloat(Integer) (- (* (Math|Conversions|ToInteger(Boolean) (Math|Random|RandomBool)) 2) 1)) 4.0) (* (Math|Random|RandomFloatinRange 0.8 1.2) 4.0))))

(event EventEventHideUnitAfterFewSeconds
  (|CallParentFunction)
  (Transformation|SetRelativeScale3D (Variables|Default|GetStaticMesh) "0, 0, 0"))

(fn ConstructionScript
  (|CallParentFunction))