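; BP_CircularSawShape is an animated spell shape component that presents a spinning circular saw.
; Each tick advances the static mesh's world yaw by RotationSpeed scaled by delta time, keeping roll and pitch unchanged.
; When the shape animation completes, it activates its Niagara effect, while construction only runs the parent script.
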(event EventTick
  (params (DeltaSeconds :type Float%20%28single-precision%29))
  (bind _staticmesh (Variables|Default|GetStaticMesh))
  (bind _returnvalue (Transformation|GetWorldRotation _staticmesh))
  (Transformation|SetWorldRotation _staticmesh (Math|Rotator|MakeRotator (.roll _returnvalue) (.pitch _returnvalue) (+ (.yaw _returnvalue) (* DeltaSeconds (Variables|Default|GetRotationSpeed)))) false false))

(fn ConstructionScript
  (|CallParentFunction))

(fn AnimationComplete
  (Components|Activation|Activate (Variables|Default|GetNiagara) false))