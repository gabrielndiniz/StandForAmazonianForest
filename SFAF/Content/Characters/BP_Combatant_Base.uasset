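; Base actor for units in tile-grid tactical combat, with team, HP, AP, MP, spell casting, death and hover/selection highlighting.
; A timeline walks paths tile by tile, spending MP; movement, idle and attack hooks are empty stubs.
; Spell impacts are queued by animation and applied on tile hit, driving health bar and floating numbers.
; Stat changes rebuild the unit struct and broadcast; dead units are moved far off-map after a delay, not destroyed.
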(event Custom|Event_FollowPath
  (params (Path :type Array%20of%20Int%20Point%20Structures) (FindPath :type BP%20Action%20Find%20Path%20to%20Target%20Object%20Reference))
  (Variables|Default|SetFind%20Path FindPath)
  (if (Utilities|Array|IsNotEmpty Path)
    (Variables|Default|SetCurrentPathToFollow Path)
    (Utilities|FlowControl|Sequence
      (:then_0
        (CallFunction|MovingAnimation))
      (:then_1
        (CallFunction|ContinuetoFollowPath)))))

(event Custom|ContinueToFollowPath
  (if (Utilities|Array|IsNotEmpty (Variables|Default|GetCurrentPathToFollow))
    (Default|CallOnUnitStartWalking self (Variables|Default|GetPosition))
    (|FollowPath)
    (else
      (CallFunction|BacktoIdle)
      (Default|CallOnUnitFinishedWalking self)
      (SettersAndGetters|SetSelectedTile))))

(event Custom|Attack
  (params (Target%20Position :type Int%20Point%20Structure)))

(event Custom|UnitHitBySpell
  (params (Impact%20Result :type ST%20Spell%20Data%20Impact%20Result%20Structure) (Spell%20Animation :type BP%20Spell%20Animation%20Object%20Reference))
  (Utilities|Map|Add (Variables|Default|GetIncomingSpellImpacts) Spell%20Animation Impact%20Result)
  (EventDispatchers|BindEventtoOnSpellHitTile Spell%20Animation (delegate Custom|OnSpellAnimationHitTile)))

(event Custom|OnSpellAnimationHitTile
  (params (SpellAnimation :type BP%20Spell%20Animation%20Object%20Reference) (Position :type Int%20Point%20Structure))
  (bind _animatednumber (Variables|Default|GetAnimatedNumber))
  (bind _incomingspellimpacts (Variables|Default|GetIncomingSpellImpacts))
  (bind (_value _returnvalue) (Utilities|Map|Find _incomingspellimpacts SpellAnimation))
  (bind _modifier_hp (Utilities|Struct|BreakST_SpellData_Impact_Result _value))
  (Utilities|FlowControl|Sequence
    (:then_0
      (if (and _returnvalue (Variables|Default|GetbIsAlive))
        (if (!= _modifier_hp 0)
          (CallFunction|ModifyCurrentHP _modifier_hp)
          (Widget|SetVisibility _animatednumber "Visible")
          (Default|ColorOfNumber _animatednumber "NewEnumerator0")
          (Default|EventPlayAnimatedNumberAnimation _animatednumber _modifier_hp)
          (if (> (.HP_Current (Utilities|Struct|BreakST_UnitData_Stats (.Stats (Utilities|Struct|BreakST_UnitData (Variables|Default|GetUnitData))))) 0)
            (CallFunction|UnitDamaged)
            (Utilities|FlowControl|Delay 1.0)
            (CallFunction|BacktoIdle)
            (else
              (CallFunction|UnitDied))))
        (else
          (Development|PrintString "Error on Combatant Base: Spell not corresponds with this target"))))
    (:then_1
      (Utilities|Map|Remove (Variables|Default|GetIncomingSpellImpacts) SpellAnimation))))

(event Custom|Event_HideUnitAfterFewSeconds
  (Utilities|FlowControl|Delay 5.0)
  (if (not (Variables|Default|GetbIsAlive))
    (Transformation|SetActorLocation "-999999.000000,-999999.000000,-999999.000000" false false)
    (for _array_element (Components|GetChildrenComponents (Variables|Default|GetDefaultSceneRoot) true)
      (Transformation|SetRelativeLocation _array_element "0, 0, 0" false false)
      (bind _asstatic_mesh_component (Utilities|Casting|CastToStaticMeshComponent _array_element))
      (Collision|SetCollisionEnabled _asstatic_mesh_component "NoCollision")
      (Physics|SetEnableGravity _asstatic_mesh_component false))))

(event EventBeginPlay
  (bind _widget_healthbar (Variables|Default|GetWidget_HealthBar))
  (CallFunction|InitiateData)
  (Transformation|SetRelativeLocation _widget_healthbar (Variables|/Script/Engine.SceneComponent|GetRelativeLocation (Variables|Default|GetBox)) false false)
  (bind _aswbp_health_bar (Utilities|Casting|CastToWBP_HealthBar (UserInterface|GetUserWidgetObject _widget_healthbar)))
  (bind _output_get (Variables|Default|SetHealthBar _aswbp_health_bar))
  (Default|EventSetUnit _output_get self)
  (bind _aswbp_animated_number (Utilities|Casting|CastToWBP_AnimatedNumber (UserInterface|GetUserWidgetObject (Variables|Default|GetWidget_AnimatedNumber))))
  (bind _output_get_2 (Variables|Default|SetAnimatedNumber _aswbp_animated_number))
  (Widget|SetVisibility _output_get_2 "Hidden"))

(event EventOnReset
  (bind _widget_healthbar (Variables|Default|GetWidget_HealthBar))
  (CallFunction|InitiateData)
  (Transformation|SetRelativeLocation _widget_healthbar (Variables|/Script/Engine.SceneComponent|GetRelativeLocation (Variables|Default|GetBox)) false false)
  (bind _aswbp_health_bar (Utilities|Casting|CastToWBP_HealthBar (UserInterface|GetUserWidgetObject _widget_healthbar)))
  (bind _output_get (Variables|Default|SetHealthBar _aswbp_health_bar))
  (Default|EventSetUnit _output_get self)
  (bind _aswbp_animated_number (Utilities|Casting|CastToWBP_AnimatedNumber (UserInterface|GetUserWidgetObject (Variables|Default|GetWidget_AnimatedNumber))))
  (bind _output_get_2 (Variables|Default|SetAnimatedNumber _aswbp_animated_number))
  (Widget|SetVisibility _output_get_2 "Hidden"))

(fn ConstructionScript)

(fn SetTeam
  (params (Team :type Byte))
  (bind _output_get (Variables|Default|SetTeam Team))
  (Class|ProgressBar|SetFillColorandOpacity (Variables|/Game/Widgets/Blueprint/Unit/UnitComponent/WBP_HealthBar.WBP_HealthBar_C|GetProgressBar_0 (Variables|Default|GetHealthBar)) (CallFunction|GetTeamColor _output_get)))

(fn GetTeam
  (return (Variables|Default|GetTeam)))

(fn GetUnitType
  (return (.type (Variables|Default|GetUnitData))))

(fn GetPosition
  (return (Variables|Default|GetPosition)))

(fn SetPosition
  (params (Position :type Int%20Point%20Structure))
  (Variables|Default|SetPosition Position))

(fn GotoLocation
  (params (NewLocation :type Vector))
  (Transformation|SetActorLocation NewLocation false false))

(fn UpdateVisualifHoveredorSelected
  (bind _bishovered (Variables|Default|GetbIsHovered))
  (bind _bisselected (Variables|Default|GetbIsSelected))
  (bind _returnvalue (select _bisselected 5.0 1.0))
  (bind _returnvalue_2 (select _bishovered 5.0 1.0))
  (bind _returnvalue_3 (* "1.000000,1.000000,1.000000" _returnvalue_2))
  (bind _returnvalue_4 (* _returnvalue_3 _returnvalue))
  (for _array_element (Components|GetChildrenComponents (Variables|Default|GetDefaultSceneRoot) true)
    (bind _asskeletal_mesh_component (Utilities|Casting|CastToSkeletalMeshComponent _array_element)
      (:then
        (Rendering|Material|SetVectorParameterValueonMaterials _asskeletal_mesh_component "ColorMultiplier" _returnvalue_4))
      (:CastFailed
        (bind _asmesh_component (Utilities|Casting|CastToMeshComponent _array_element))
        (Rendering|Material|SetVectorParameterValueonMaterials _asmesh_component "ColorMultiplier" _returnvalue_4)))))

(fn SetIsHovered
  (params (bIsHovered :type Boolean))
  (Variables|Default|SetbIsHovered bIsHovered)
  (CallFunction|UpdateVisualifHoveredorSelected))

(fn SetIsSelected
  (params (bIsSelected :type Boolean))
  (Variables|Default|SetbIsSelected bIsSelected)
  (CallFunction|UpdateVisualifHoveredorSelected))

(fn GetUnitData
  (return (Variables|Default|GetUnitData)))

(fn SetGrid
  (params (Grid :type BP%20Grid%20Object%20Reference))
  (Variables|Default|SetGrid Grid))

(fn MovingAnimation)

(fn BacktoIdle)

(fn SetMoveSpeed
  (params (MoveDurationPerTile :type Float%20%28double-precision%29))
  (Variables|Default|SetMoveSpeed MoveDurationPerTile))

(fn InitiateData
  (bind _unit_data (CallFunction|GetDefaultUnitDatafromUnitType (.type (Variables|Default|GetUnitData))))
  (SettersAndGetters|SetUnitData _unit_data))

(fn UnitCastSpell
  (params (TargetPosition :type Int%20Point%20Structure) (SpellDataRequirements :type ST%20Spell%20Data%20Requirements%20Structure))
  (bind _returnvalue (Transformation|GetActorLocation))
  (bind _grid (Variables|Default|GetGrid))
  (bind _tiledata (Default|GetTileData _grid TargetPosition))
  (Transformation|SetActorRotation (Math|Rotator|FindLookatRotation (Math|Vector|MakeVector (.x _returnvalue) (.y _returnvalue) 0.0) (Math|Vector|MakeVector (.x (.location (.transform _tiledata))) (.y (.location (.transform _tiledata))) 0.0)))
  (CallFunction|Attack)
  (CallFunction|ModifyCurrentAP (* (Utilities|Struct|BreakST_SpellData_Requirements SpellDataRequirements) -1) true))

(fn ModifyCurrentHP
  (params (Modifier :type Integer))
  (SettersAndGetters|SetCurrentHP (+ Modifier (.HP_Current (Utilities|Struct|BreakST_UnitData_Stats (.stats (Variables|Default|GetUnitData)))))))

(fn SetCurrentHP
  (params (HP :type Integer))
  (bind _unitdata (Variables|Default|GetUnitData))
  (bind (_validtiletypes _movementpoints_current _movementpoints_max _availablespells _hp_current _hp_max _ap_current _ap_max) (Utilities|Struct|BreakST_UnitData_Stats (.stats _unitdata)))
  (SettersAndGetters|SetUnitData (Utilities|Struct|MakeST_UnitData (.type _unitdata) (.assets _unitdata) (Utilities|Struct|MakeST_UnitData_Stats _validtiletypes _movementpoints_current _movementpoints_max _availablespells (Math|Integer|Clamp(Integer) HP 0 _hp_max) _hp_max _ap_current _ap_max)))
  (Default|CallOnUnitStatsChanged self))

(fn UnitDamaged
  (Default|EventUpdateBar (Variables|Default|GetHealthBar)))

(fn UnitDied
  (bind _unitdata (Variables|Default|GetUnitData))
  (bind (_type _assets _stats) (Utilities|Struct|BreakST_UnitData _unitdata))
  (Variables|Default|SetbIsAlive false)
  (SettersAndGetters|SetUnitData (Utilities|Struct|MakeST_UnitData _type _assets (Utilities|Struct|MakeST_UnitData_Stats (.validtiletypes _stats) 0 0 (Utilities|Array|MakeArray) 0 (.hp_max _stats) 0 (.ap_max _stats))))
  (Components|DestroyComponent (Variables|Default|GetBox))
  (Rendering|SetVisibility (Variables|Default|GetWidget_HealthBar) false false)
  (CallFunction|EventHideUnitAfterFewSeconds)
  (Default|CallOnUnitDeath self))

(fn CombatStarted
  (Development|PrintString (Utilities|String|Append (Utilities|GetObjectName self) " is in combat."))
  (CallFunction|ResetMP)
  (CallFunction|ResetAP))

(fn TurnStarted
  (Development|PrintString (Utilities|String|Append (Utilities|GetObjectName self) " is in his turn.")))

(fn TurnEnded
  (Development|PrintString (Utilities|String|Append (Utilities|GetObjectName self) " ended his turn."))
  (CallFunction|ResetMP)
  (CallFunction|ResetAP))

(fn CombatEnded
  (Development|PrintString (Utilities|String|Append (Utilities|GetObjectName self) " ended the combat."))
  (CallFunction|ResetMP)
  (CallFunction|ResetAP))

(fn ModifyCurrentMP
  (params (Modifier :type Integer) (bShowNumber :type Boolean))
  (SettersAndGetters|SetCurrentMP (+ Modifier (.MovementPoints_Current (Utilities|Struct|BreakST_UnitData_Stats (.Stats (Utilities|Struct|BreakST_UnitData (Variables|Default|GetUnitData)))))) bShowNumber))

(fn SetCurrentMP
  (params (MovementPoints :type Integer) (bShowNumber :type Boolean))
  (bind _unitdata (Variables|Default|GetUnitData))
  (bind _animatednumber (Variables|Default|GetAnimatedNumber))
  (bind (_validtiletypes _movementpoints_current _movementpoints_max _availablespells _hp_current _hp_max _ap_current _ap_max) (Utilities|Struct|BreakST_UnitData_Stats (.stats _unitdata)))
  (LocalVariables|SetDifference (- MovementPoints (.MovementPoints_Current (Utilities|Struct|BreakST_UnitData_Stats (.Stats (Utilities|Struct|BreakST_UnitData (Variables|Default|GetUnitData)))))))
  (SettersAndGetters|SetUnitData (Utilities|Struct|MakeST_UnitData (.type _unitdata) (.assets _unitdata) (Utilities|Struct|MakeST_UnitData_Stats _validtiletypes (Math|Integer|Clamp(Integer) MovementPoints 0 _movementpoints_max) _movementpoints_max _availablespells _hp_current _hp_max _ap_current _ap_max)))
  (if (and bShowNumber (!= (LocalVariables|GetDifference) 0))
    (Widget|SetVisibility _animatednumber "Visible")
    (Default|ColorOfNumber _animatednumber "NewEnumerator1")
    (Default|EventPlayAnimatedNumberAnimation _animatednumber (LocalVariables|GetDifference))))

(fn ResetMP
  (SettersAndGetters|SetCurrentMP (.MovementPoints_Max (Utilities|Struct|BreakST_UnitData_Stats (.Stats (Utilities|Struct|BreakST_UnitData (Variables|Default|GetUnitData))))) false))

(fn SetSelectedTile
  ;[0.01124 0.008981 0.05729] TODO: Select the action manager according with team
  (bind _asbp_tactical_grid_controller (Utilities|Casting|CastToBP_TacticalGridController (Game|GetPlayerController 0)))
  (Default|SetSelectedTile (Variables|/Game/TopDown/Blueprints/BP_TacticalGridController.BP_TacticalGridController_C|GetBP_ActionManager _asbp_tactical_grid_controller) true (Variables|Default|GetPosition) self))

(fn ModifyCurrentAP
  (params (Modifier :type Integer) (bShowNumber :type Boolean))
  (SettersAndGetters|SetCurrentAP (+ Modifier (.AP_Current (Utilities|Struct|BreakST_UnitData_Stats (.Stats (Utilities|Struct|BreakST_UnitData (Variables|Default|GetUnitData)))))) bShowNumber))

(fn ResetAP
  (SettersAndGetters|SetCurrentAP (.AP_Max (Utilities|Struct|BreakST_UnitData_Stats (.Stats (Utilities|Struct|BreakST_UnitData (Variables|Default|GetUnitData))))) false))

(fn SetCurrentAP
  (params (ActionPoints :type Integer) (bShowNumber :type Boolean))
  (bind _unitdata (Variables|Default|GetUnitData))
  (bind _animatednumber (Variables|Default|GetAnimatedNumber))
  (bind (_validtiletypes _movementpoints_current _movementpoints_max _availablespells _hp_current _hp_max _ap_current _ap_max) (Utilities|Struct|BreakST_UnitData_Stats (.stats _unitdata)))
  (LocalVariables|SetDifference (- ActionPoints (.AP_Current (Utilities|Struct|BreakST_UnitData_Stats (.Stats (Utilities|Struct|BreakST_UnitData (Variables|Default|GetUnitData)))))))
  (SettersAndGetters|SetUnitData (Utilities|Struct|MakeST_UnitData (.type _unitdata) (.assets _unitdata) (Utilities|Struct|MakeST_UnitData_Stats _validtiletypes _movementpoints_current _movementpoints_max _availablespells _hp_current _hp_max (Math|Integer|Clamp(Integer) ActionPoints 0 _ap_max) _ap_max)))
  (if (and bShowNumber (!= (LocalVariables|GetDifference) 0))
    (Widget|SetVisibility _animatednumber "Visible")
    (Default|ColorOfNumber _animatednumber "NewEnumerator2")
    (Default|EventPlayAnimatedNumberAnimation _animatednumber (LocalVariables|GetDifference))))

(fn CanCastSpell
  (params (SpellData :type ST%20Spell%20Data%20Structure))
  (if (Utilities|Array|ContainsItem (.AvailableSpells (Utilities|Struct|BreakST_UnitData_Stats (.Stats (Utilities|Struct|BreakST_UnitData (Variables|Default|GetUnitData))))) (.Spell (Utilities|Struct|BreakST_SpellData SpellData)))
    (if (>= (.AP_Current (Utilities|Struct|BreakST_UnitData_Stats (.Stats (Utilities|Struct|BreakST_UnitData (Variables|Default|GetUnitData))))) (Utilities|Struct|BreakST_SpellData_Requirements (.Requirements (Utilities|Struct|BreakST_SpellData SpellData))))
      (return true)
      (else
        (return false)))
    (else
      (return false))))

(fn SetUnitData
  (params (UnitData :type ST%20Unit%20Data%20Structure))
  (Variables|Default|SetUnitData UnitData)
  (Default|CallOnUnitStatsChanged self))

(fn GetIsAlive
  (return (Variables|Default|GetbIsAlive)))