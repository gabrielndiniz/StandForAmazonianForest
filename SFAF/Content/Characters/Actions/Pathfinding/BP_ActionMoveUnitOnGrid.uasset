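; Grid action that moves the unit on a given tile along a path from an assigned pathfinding object.
; ExecuteAction runs the parent action, then hands the FindPathToMove path to the tile's unit through EventFollowPath if the path is non-empty and valid.
; BeginPlay retries until the Grid is valid, then derives MaxExpectedInteractions from the grid's last position as an infinite-loop safeguard.
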(event EventBeginPlay
  (bind _grid (Variables|Default|GetGrid))
  (bind _gridlastposition (Default|GetGridLastPosition _grid))
  (|CallParentFunction)
  (Utilities|IsValid (Variables|Default|GetGrid) :!label _label
    (:Is%20Valid
      ;[0.04688 0.04688 0.04688] To reduce chance of infinite loop.
      (Variables|Default|SetMaxExpectedInteractions (+ (.x _gridlastposition) (.y _gridlastposition))))
    (:Is%20Not%20Valid
      (Utilities|FlowControl|Delay 2.0)
      (goto _label))))

(event Collision|EventActorBeginOverlap
  (params (OtherActor :type Actor%20Object%20Reference))
  (|CallParentFunction OtherActor) ; This node is disabled and will not be called.\nDrag off pins to build functionality.
)

(event EventTick
  (params (DeltaSeconds :type Float%20%28single-precision%29))
  (|CallParentFunction DeltaSeconds) ; This node is disabled and will not be called.\nDrag off pins to build functionality.
)

(fn ConstructionScript
  (|CallParentFunction))

(fn ExecuteAction
  (params (Position%201 :type Int%20Point%20Structure) (bHitResult :type Boolean) (Position%202 :type Int%20Point%20Structure))
  (bind _grid (Variables|Default|GetGrid))
  (bind _findpathtomove (Variables|Default|GetFindPathToMove))
  (bind _tiledata (Default|GetTileData _grid Position%201))
  (bind _path (Default|GetPath _findpathtomove))
  (bind (_success _tiledata1 _tiledata2) (|CallParentFunction Position%201 bHitResult Position%202))
  (Utilities|IsValid (Variables|Default|GetGrid)
    (:Is%20Valid
      (Utilities|FlowControl|Sequence
        (:then_0
          (if (Utilities|Array|IsNotEmpty _path)
            (if (and (Utilities|IsValid (.unitontyle _tiledata)) (> (.x (Utilities|Array|Get(acopy) _path)) -999))
              (Default|EventFollowPath (.unitontyle _tiledata) _path (Variables|Default|GetFindPathToMove)))))
        (:then_1
          (return _success _tiledata1 _tiledata2))))
    (:Is%20Not%20Valid
      (return false "" ""))))

(fn SetFindPath
  (params (FindPath :type BP%20Action%20Find%20Path%20to%20Target%20Object%20Reference))
  (Variables|Default|SetFindPathToMove FindPath))

(fn GetPath
  (return (Variables|Default|GetPath)))