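; BP_GridModifier is a grid marker actor that carries a tile type (such as Obstacle, DoubleCost or FlyingUnitsOnly) and a height-use flag, exposed through getters.
; Construction gives its hexagon the grid shape's solid mesh, colors it by type with adjustable glow and opacity, and sets overlap on a custom trace channel.
; BeginPlay hides the hexagon in game; SetTacticalMode is an empty stub.
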(event EventBeginPlay
  (Development|SetHiddeninGame (Variables|Default|GetSolidHexagon) true false))

(event Collision|EventActorBeginOverlap
  (params (OtherActor :type Actor%20Object%20Reference)))

(event EventTick
  (params (DeltaSeconds :type Float%20%28single-precision%29)))

(fn ConstructionScript
  (bind _solidhexagon (Variables|Default|GetSolidHexagon))
  (Components|StaticMesh|SetStaticMesh _solidhexagon (.Solid (Default|GetShapeData (Variables|Default|GetBP_GridDataComponent))))
  (Rendering|Material|SetVectorParameterValueonMaterials _solidhexagon "Color" (Math|Conversions|ToVector(LinearColor) (Utilities|Select :Index (Variables|Default|GetType) :NewEnumerator0 "(R=0.000000,G=1.000000,B=0.000000,A=1.000000)" :NewEnumerator1 "(R=0.000000,G=0.000000,B=0.000000,A=1.000000)" :NewEnumerator2 "(R=1.000000,G=0.000000,B=0.839263,A=1.000000)" :NewEnumerator3 "(R=0.132568,G=1.000000,B=0.000000,A=1.000000)" :NewEnumerator4 "(R=1.000000,G=0.025978,B=0.000000,A=1.000000)" :NewEnumerator5 "(R=0.000000,G=0.029868,B=1.000000,A=1.000000)")))
  ;[1 1 1] This segment will decide if there will be color or not on the StaticMesh. It will bright from inside, not from outside.
  (Rendering|Material|SetScalarParameterValueonMaterials _solidhexagon "MultiplierForEmissionAndOpacity" (Variables|Default|GetBrightMultiply))
  (Rendering|Material|SetScalarParameterValueonMaterials _solidhexagon "AddAfterMultiplier" (Variables|Default|GetBrightAdder))
  (Collision|SetCollisionResponsetoChannel (Variables|Default|GetSolidHexagon) "ECC_GameTraceChannel3" "ECR_Overlap")
  (Development|SetHiddeninGame (Variables|Default|GetSolidHexagon) false false))

(fn GetTileType
  (return (Variables|Default|GetType)))

(fn GetUseforHeight
  (return (Variables|Default|GetbUseForHeight)))

(fn SetTacticalMode
  (params (Tactical%20Mode :type Boolean)))