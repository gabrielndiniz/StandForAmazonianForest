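; Grid action that finds the valid neighbors of a selected tile, flags them with a tile state and can display them as instanced meshes.
; When the position changes, it clears the previous set, then on a hit gathers up to eight existing neighbors using row-parity offsets for a staggered grid.
; The mesh display is toggleable and is rebuilt inside the per-neighbor loop.
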(event EventBeginPlay
  (|CallParentFunction) ; This node is disabled and will not be called.\nDrag off pins to build functionality.
)

(event Collision|EventActorBeginOverlap
  (params (OtherActor :type Actor%20Object%20Reference))
  (|CallParentFunction OtherActor) ; This node is disabled and will not be called.\nDrag off pins to build functionality.
)

(event EventTick
  (params (DeltaSeconds :type Float%20%28single-precision%29))
  (|CallParentFunction DeltaSeconds) ; This node is disabled and will not be called.\nDrag off pins to build functionality.
)

(fn ConstructionScript
  (|CallParentFunction))

(fn ExecuteAction
  (params (Position :type Int%20Point%20Structure) (bHitResult :type Boolean))
  (bind (_success _tiledata) (|CallParentFunction Position bHitResult))
  (Utilities|FlowControl|Sequence
    (:then_0
      (if (!= Position (Variables|Default|GetCurrentPositon))
        (CallFunction|ClearTiles)
        (if bHitResult
          (bind _output_get (Variables|Default|SetCurrentPositon Position))
          (CallFunction|SetValidTileNeighbors _output_get)
          (for _array_element (Variables|Default|GetNeighborPositions)
            (Default|AddStateTile (Variables|Default|GetGrid) _array_element "NewEnumerator3")
            (CallFunction|ShowNeighbors))
          (else
            (Variables|Default|SetCurrentPositon (Utilities|Struct|MakeIntPoint 9999 9999))))))
    (:then_1
      (return _success _tiledata))))

(fn SetShowNeighbors
  (params (bShowNeighbors :type Boolean))
  (Variables|Default|SetbShowNeighbors bShowNeighbors))

(fn ShowNeighbors
  (Components|InstancedStaticMesh|ClearInstances (Variables|Default|GetInstancedStaticMesh))
  (if (Variables|Default|GetbShowNeighbors)
    (for _array_element (Variables|Default|GetNeighborPositions)
      (Components|InstancedStaticMesh|AddInstance (Variables|Default|GetInstancedStaticMesh) (.transform (.TileData (Default|GetTileData (Variables|Default|GetGrid) _array_element))) true))))

(fn SetValidTileNeighbors
  (params (Position :type Int%20Point%20Structure))
  (bind _grid (Variables|Default|GetGrid))
  (bind _tiledata (Default|GetTileData _grid Position))
  (LocalVariables|SetXValue (.x (.position _tiledata)))
  (LocalVariables|SetYValue (.y (.position _tiledata)))
  (for _index (range 0 1)
    (bind _output_get (LocalVariables|SetAddPosition (Utilities|Struct|MakeIntPoint (LocalVariables|GetXValue) (+ (* _index 4) -2 (LocalVariables|GetYValue)))))
    (if (.Success (Default|GetTileData (Variables|Default|GetGrid) _output_get))
      (Utilities|Array|Add (Variables|Default|GetNeighborPositions) (LocalVariables|GetAddPosition))))
  (if (CallFunction|IsIntEven (LocalVariables|GetYValue))
    (LocalVariables|SetAddPosition (Utilities|Struct|MakeIntPoint (- (LocalVariables|GetXValue) 1) (LocalVariables|GetYValue)))
    (if (.Success (Default|GetTileData (Variables|Default|GetGrid) (LocalVariables|GetAddPosition)))
      (Utilities|Array|Add (Variables|Default|GetNeighborPositions) (LocalVariables|GetAddPosition)))
    (for _index_2 (range (LocalVariables|GetXValue) (+ (LocalVariables|GetXValue) 1))
      (for _index_3 (range (- (LocalVariables|GetYValue) 1) (+ (LocalVariables|GetYValue) 1))
        (LocalVariables|SetAddPosition (Utilities|Struct|MakeIntPoint _index_2 _index_3))
        (if (and (.Success (Default|GetTileData (Variables|Default|GetGrid) (LocalVariables|GetAddPosition))) (!= Position (LocalVariables|GetAddPosition)))
          (Utilities|Array|Add (Variables|Default|GetNeighborPositions) (LocalVariables|GetAddPosition)))))
    (else
      (LocalVariables|SetAddPosition (Utilities|Struct|MakeIntPoint (+ (LocalVariables|GetXValue) 1) (LocalVariables|GetYValue)))
      (if (.Success (Default|GetTileData (Variables|Default|GetGrid) (LocalVariables|GetAddPosition)))
        (Utilities|Array|Add (Variables|Default|GetNeighborPositions) (LocalVariables|GetAddPosition)))
      (for _index_4 (range (- (LocalVariables|GetXValue) 1) (LocalVariables|GetXValue))
        (for _index_5 (range (- (LocalVariables|GetYValue) 1) (+ (LocalVariables|GetYValue) 1))
          (LocalVariables|SetAddPosition (Utilities|Struct|MakeIntPoint _index_4 _index_5))
          (if (and (.Success (Default|GetTileData (Variables|Default|GetGrid) (LocalVariables|GetAddPosition))) (!= Position (LocalVariables|GetAddPosition)))
            (Utilities|Array|Add (Variables|Default|GetNeighborPositions) (LocalVariables|GetAddPosition))))))))

(fn ClearTiles
  (for _array_element (Variables|Default|GetNeighborPositions)
    (Default|RemoveStateTile (Variables|Default|GetGrid) _array_element "NewEnumerator3"))
  (Utilities|Array|Clear (Variables|Default|GetNeighborPositions))
  (Components|InstancedStaticMesh|ClearInstances (Variables|Default|GetInstancedStaticMesh)))

(fn GetValidTileNeighbors
  (return (Variables|Default|GetNeighborPositions)))