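; BP_ActionSelectTile is an action actor that marks a selected tile with a glowing cyan hexagon.
; ExecuteAction calls the parent action and, on success, moves the hexagon to the returned tile's location.
; ChangeHexagonColor pulses emission and opacity through material parameters, reversing speed at the bounds and shifting the multiplier opposite to the adder.
; Construction sets the initial color and brightness; nothing in this graph calls the pulse function.
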(event EventBeginPlay
  (|CallParentFunction) ; This node is disabled and will not be called.\nDrag off pins to build functionality.
)

(event Collision|EventActorBeginOverlap
  (params (OtherActor :type Actor%20Object%20Reference))
  (|CallParentFunction OtherActor) ; This node is disabled and will not be called.\nDrag off pins to build functionality.
)

(event EventTick
  (params (DeltaSeconds :type Float%20%28single-precision%29))
  (|CallParentFunction DeltaSeconds) ; This node is disabled and will not be called.\nDrag off pins to build functionality.
)

(fn ConstructionScript
  (bind _hexagon (Variables|Default|GetHexagon))
  (|CallParentFunction)
  (Rendering|Material|SetVectorParameterValueonMaterials _hexagon "Color" (Math|Conversions|ToVector(LinearColor) (Math|Color|MakeColor 0.07 0.8 0.9)))
  (Rendering|Material|SetScalarParameterValueonMaterials _hexagon "MultiplierForEmissionAndOpacity" (Variables|Default|GetBrightMultiply))
  (Rendering|Material|SetScalarParameterValueonMaterials _hexagon "AddAfterMultiplier" (Variables|Default|GetBrightAdder)))

(fn SetHexagonLocation
  (params (NewLocation :type Vector))
  (Transformation|SetWorldLocation (Variables|Default|GetHexagon) NewLocation false false))

(fn ExecuteAction
  (params (Index :type Integer))
  (bind (_success _tiledata) (|CallParentFunction Index))
  (bind _output_get (LocalVariables|SetContinue _success))
  (if _output_get
    (bind _output_get_2 (LocalVariables|SetData _tiledata))
    (CallFunction|SetHexagonLocation (.location (.transform _output_get_2))))
  (return (LocalVariables|GetContinue) (LocalVariables|GetData)))

(fn ChangeHexagonColor
  (bind _hexagon (Variables|Default|GetHexagon))
  (Rendering|Material|SetScalarParameterValueonMaterials _hexagon "MultiplierForEmissionAndOpacity" (Variables|Default|GetBrightMultiply))
  (Rendering|Material|SetScalarParameterValueonMaterials _hexagon "AddAfterMultiplier" (Variables|Default|GetBrightAdder))
  (if (or (>= (Variables|Default|GetBrightAdder) 1.0) (<= (Variables|Default|GetBrightAdder) 0.0))
    (Variables|Default|SetChangeColorSpeed (* (Variables|Default|GetChangeColorSpeed) -1.0)))
  (Variables|Default|SetBrightAdder (+ (* (Variables|Default|GetChangeColorSpeed) (Utilities|Time|GetWorldDeltaSeconds)) (Variables|Default|GetBrightAdder)))
  (Variables|Default|SetBrightMultiply (+ (* (* (Variables|Default|GetChangeColorSpeed) (Utilities|Time|GetWorldDeltaSeconds)) -2.0) (Variables|Default|GetBrightMultiply))))