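; BP_WaitForTurn is a combat action that switches player control on or off, apparently around turn waits.
; Its ExecuteAction override calls the parent, then uses HitResult as a flag to toggle pawn and controller input and the mouse cursor.
; It returns the parent's success and tile data.
; A separate ActivatePlayerCamera function, not called here, forwards an activate flag to the BP_PlayerCamera pawn.
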(event EventBeginPlay
  (|CallParentFunction) ; This node is disabled and will not be called.\nDrag off pins to build functionality.
)

(event Collision|EventActorBeginOverlap
  (params (OtherActor :type Actor%20Object%20Reference))
  (|CallParentFunction OtherActor) ; This node is disabled and will not be called.\nDrag off pins to build functionality.
)

(event EventTick
  (params (DeltaSeconds :type Float%20%28single-precision%29)))

(fn ConstructionScript
  (|CallParentFunction))

(fn ExecuteAction
  (params (Position%201 :type Int%20Point%20Structure) (bHitResult :type Boolean) (Position%202 :type Int%20Point%20Structure))
  (bind (_success _tiledata1 _tiledata2) (|CallParentFunction Position%201 bHitResult Position%202))
  (Utilities|FlowControl|Sequence
    (:then_0
      (if bHitResult
        (bind _asplayer_controller (Utilities|Casting|CastToPlayerController (Variables|Default|GetController)))
        (Input|EnableInput (Variables|Default|GetPawn) _asplayer_controller)
        (Input|EnableInput _asplayer_controller _asplayer_controller)
        (Variables|/Script/Engine.PlayerController|SetbShowMouseCursor _asplayer_controller true)
        (else
          (bind _asplayer_controller_2 (Utilities|Casting|CastToPlayerController (Variables|Default|GetController)))
          (Input|DisableInput (Variables|Default|GetPawn) _asplayer_controller_2)
          (Input|DisableInput _asplayer_controller_2 _asplayer_controller_2)
          (Variables|/Script/Engine.PlayerController|SetbShowMouseCursor _asplayer_controller_2 false))))
    (:then_1
      (return _success _tiledata1 _tiledata2))))

(fn ActivatePlayerCamera
  (params (bActivate :type Boolean))
  (Utilities|Casting|CastToPlayerController (Variables|Default|GetController))
  (bind _asbp_player_camera (Utilities|Casting|CastToBP_PlayerCamera (Variables|Default|GetPawn)))
  (Default|ActivateCamera _asbp_player_camera bActivate))