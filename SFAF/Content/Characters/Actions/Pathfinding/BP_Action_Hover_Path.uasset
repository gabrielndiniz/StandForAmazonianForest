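; Hover action that previews the path between two grid positions for the unit standing on the first tile.
; ExecuteAction runs the parent action, then passes that tile's unit to GenerateReachable, which clears the old preview and, if the unit is valid, queries the assigned FindPath object.
; Each tile on a found path gets an instanced static mesh at its grid transform, raised slightly above the tile.
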(fn ConstructionScript
  (|CallParentFunction))

(fn GenerateReachable
  (params (Unit :type BP%20Combatant%20Base%20Object%20Reference) (Position1 :type Int%20Point%20Structure) (Position2 :type Int%20Point%20Structure))
  (if (!= Unit (Variables|Default|GetCurrentUnit))
    (Variables|Default|SetCurrentUnit Unit))
  (CallFunction|ClearPath)
  (Utilities|IsValid (Variables|Default|GetCurrentUnit)
    (:Is%20Valid
      (bind (_path _bfoundpath) (Default|FindPath (Variables|Default|GetFindPath) Position1 Position2 false false false))
      (if _bfoundpath
        (for _array_element _path
          (Components|InstancedStaticMesh|AddInstance (Variables|Default|GetInstancedStaticMeshPath) (Math|Transform|MakeTransform (Math|Vector|MakeVector (.x (.location (.transform (.TileData (Default|GetTileData (Variables|Default|GetGrid) _array_element))))) (.y (.location (.transform (.TileData (Default|GetTileData (Variables|Default|GetGrid) _array_element))))) (+ (.z (.location (.transform (.TileData (Default|GetTileData (Variables|Default|GetGrid) _array_element))))) 5.0)) (.rotation (.transform (.TileData (Default|GetTileData (Variables|Default|GetGrid) _array_element)))) (.scale (.transform (.TileData (Default|GetTileData (Variables|Default|GetGrid) _array_element))))) true))))))

(fn SetFindPathtoTarget
  (params (FindPath :type BP%20Action%20Find%20Path%20to%20Target%20Object%20Reference))
  (Variables|Default|SetFindPath FindPath))

(fn ExecuteAction
  (params (Position%201 :type Int%20Point%20Structure) (bHitResult :type Boolean) (Position%202 :type Int%20Point%20Structure))
  (bind (_success _tiledata1 _tiledata2) (|CallParentFunction Position%201 bHitResult Position%202))
  (Utilities|FlowControl|Sequence
    (:then_0
      (CallFunction|GenerateReachable (.UnitOnTyle (Utilities|Struct|BreakST_TileData _tiledata1)) Position%201 Position%202))
    (:then_1
      (return _success _tiledata1 _tiledata2))))

(fn ClearPath
  (Components|InstancedStaticMesh|ClearInstances (Variables|Default|GetInstancedStaticMeshPath)))