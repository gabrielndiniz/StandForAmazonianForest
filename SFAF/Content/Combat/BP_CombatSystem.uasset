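; Combat manager for a grid-based, turn-based game that registers units, tracks teams and runs combat until one team remains.
; It syncs unit positions with BP_Grid tile data, destroying units on tiles that become unwalkable.
; Turns follow team order: a team's player units act together, while AI units, driven by spawned BP_AIPawns, act singly.
; Spell casts spawn data-driven range, AOE and effect actors and apply randomized impacts to target units.
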(event Custom|Event_ProcessUnitDeath
  (params (Unit :type BP%20Combatant%20Base%20Object%20Reference))
  (bind (_bcontinue _liveteam) (CallFunction|HaveEnoughTeamstoContinue))
  (Utilities|FlowControl|Delay 0.2)
  (Combatant|RemoveUnitfromTile (Default|GetPosition Unit) Unit true false)
  (Utilities|FlowControl|Sequence
    (:then_0
      (Utilities|FlowControl|Delay 5.0)
      (CallFunction|SetLocationOfUnit (Utilities|Struct|MakeIntPoint -999 -999) Unit))
    (:then_1
      (if (not _bcontinue)
        (Development|PrintString "combat ended")
        (CallFunction|HaveWinningTeam _liveteam)
        (else
          (Development|PrintString "combat continue"))))))

(event Custom|Event%20OnTileStateUpdate
  (params (Position :type Int%20Point%20Structure))
  (CallFunction|OnTileDataUpdated Position))

(event Custom|Event%20UnitChanged
  (Default|CallOnUnitTeamChanged))

(event Custom|Event%20OnGridModified
  (Utilities|FlowControl|Delay 2.0)
  (CallFunction|OnGridDestroyed))

(event EventBeginPlay
  (Utilities|FlowControl|Delay 1.0 :!label _label)
  (bind _returnvalue (Actor|GetActorOfClass "/Game/Ground/Terrain/BP_Grid.BP_Grid_C"))
  (bind _output_get (Variables|Default|SetGrid _returnvalue))
  (Utilities|IsValid _output_get
    (:Is%20Valid
      (EventDispatchers|BindEventtoOnGridDestroyed (Variables|Default|GetGrid) (delegate Custom|Event%20OnGridModified))
      (EventDispatchers|BindEventtoOnTileDataUpdated (Variables|Default|GetGrid) (delegate Custom|Event%20OnTileStateUpdate)))
    (:Is%20Not%20Valid
      (goto _label))))

(fn ConstructionScript)

(fn AddUnitinCombat
  (params (Unit :type BP%20Combatant%20Base%20Object%20Reference) (Position :type Int%20Point%20Structure) (bAIUnit :type Boolean))
  (Utilities|Array|Add (Variables|Default|GetUnits) Unit)
  (Combatant|SetUnitPositiononGrid Unit Position false false true)
  (EventDispatchers|BindEventtoOnUnitStartWalking Unit (EventDispatchers|CreateEvent :!event OnUnitStartWalking))
  (EventDispatchers|BindEventtoOnUnitReachedNewTile Unit (EventDispatchers|CreateEvent :!event OnUnitReachedNewTile))
  (EventDispatchers|BindEventtoOnUnitFinishedWalking Unit (EventDispatchers|CreateEvent :!event OnUnitFinishedPath))
  (Combatant|SetUnitUseAI Unit bAIUnit))

(fn RemoveUnitfromCombat
  (params (Unit :type BP%20Combatant%20Base%20Object%20Reference) (DestroyUnit :type Boolean))
  (Utilities|Array|RemoveItem (Variables|Default|GetUnits) Unit)
  (Utilities|IsValid Unit
    (:Is%20Valid
      (Combatant|SetUnitPositiononGrid Unit (Utilities|Struct|MakeIntPoint 99999 99999) false false true)
      (if DestroyUnit
        (Actor|DestroyActor Unit)))))

(fn SetUnitPositiononGrid
  (params (Unit :type BP%20Combatant%20Base%20Object%20Reference) (Position :type Int%20Point%20Structure) (Force%20Remove :type Boolean) (Force%20Move :type Boolean) (AffectLocation :type Boolean))
  (Utilities|IsValid Unit
    (:Is%20Valid
      (if (or (!= (Default|GetPosition Unit) Position) Force%20Move)
        (Utilities|FlowControl|Sequence
          (:then_0
            ;[0.1562 0 0] Removing Unit on Tile Data from Previous Tile
            (Combatant|RemoveUnitfromTile Position Unit Force%20Remove true))
          (:then_1
            ;[0 0.02312 0.1771] Add Unit on Current Tile
            (Combatant|AddUnittoTile Position Unit))
          (:then_2
            ;[0.125 0.1027 0] Set the Location of the Unit
            (if AffectLocation
              (CallFunction|SetLocationOfUnit Position Unit)))
          (:then_3
            ;[0.1478 0.526 0.5156] Set Basics
            (Default|SetGrid Unit (Variables|Default|GetGrid)))
          (:then_4
            ;[0.125 0.125 0.125] Call Dispatcher
            (Default|CallOnUnitPositionChanged Unit Position)))))))

(fn OnTileDataUpdated
  (params (Position :type Int%20Point%20Structure))
  (bind _output_get (LocalVariables|SetCopyOfUnits (Variables|Default|GetUnits)))
  (for _array_element _output_get
    (Utilities|IsValid _array_element
      (:Is%20Valid
        (if (Class|KismetMathLibrary|EqualIntPointIntPoint (Default|GetPosition _array_element) Position)
          (if (Default|IsTileWalkable (Variables|Default|GetGrid) (Default|GetPosition _array_element))
            (Combatant|SetUnitPositiononGrid _array_element (Default|GetPosition _array_element) false false true)
            (else
              (Combatant|RemoveUnitfromCombat _array_element true)))
          (return)))
      (:Is%20Not%20Valid
        (Utilities|Array|RemoveItem (Variables|Default|GetUnits) _array_element)))))

(fn OnGridDestroyed
  (bind _output_get (LocalVariables|SetCopyOfUnits (Variables|Default|GetUnits)))
  (for _array_element _output_get
    (if (Default|IsTileWalkable (Variables|Default|GetGrid) (Default|GetPosition _array_element))
      (Combatant|SetUnitPositiononGrid _array_element (Default|GetPosition _array_element) false false true)
      (else
        (Combatant|RemoveUnitfromCombat _array_element true)))))

(fn RemoveUnitfromTile
  (params (Position :type Int%20Point%20Structure%20%28by%20ref%29) (Unit :type Object%20Object%20Reference) (bForce :type Boolean) (bDestroyPreviousActor :type Boolean))
  (bind _output_get (LocalVariables|SetPreviousTile (.TileData (Default|GetTileData (Variables|Default|GetGrid) Position))))
  (if (or (!= (.unitontyle _output_get) Unit) bForce)
    (Utilities|IsValid (.unitontyle _output_get)
      (:Is%20Valid
        (if bDestroyPreviousActor
          (Actor|DestroyActor (.unitontyle _output_get))))
      (:Is%20Not%20Valid
        _))
    (bind _structout (Utilities|Struct|SetmembersinST_TileData (LocalVariables|GetPreviousTile)))
    (Default|AddTileData (Variables|Default|GetGrid) (.Position (Utilities|Struct|BreakST_TileData _structout)) _structout)))

(fn AddUnittoTile
  (params (Position :type Int%20Point%20Structure) (Unit :type BP%20Combatant%20Base%20Object%20Reference))
  (Default|SetPosition Unit Position)
  (if (< (.x Position) 99999)
    (bind _structout (Utilities|Struct|SetmembersinST_TileData (.TileData (Default|GetTileData (Variables|Default|GetGrid) (Default|GetPosition Unit))) Unit))
    (Default|AddTileData (Variables|Default|GetGrid) (.Position (Utilities|Struct|BreakST_TileData _structout)) _structout)
    (EventDispatchers|BindEventtoOnUnitDeath Unit (EventDispatchers|CreateEvent :!event Custom|Event_ProcessUnitDeath))))

(fn OnUnitReachedNewTile
  (params (Unit :type BP%20Combatant%20Base%20Object%20Reference) (Location :type Int%20Point%20Structure))
  (Combatant|SetUnitPositiononGrid Unit Location false true true))

(fn OnUnitFinishedPath
  (params (Unit :type BP%20Combatant%20Base%20Object%20Reference))
  (Default|CallOnUnitFinishedWalking Unit))

(fn OnUnitStartWalking
  (params (Unit :type BP%20Combatant%20Base%20Object%20Reference) (Position :type Int%20Point%20Structure))
  (bind _grid (Variables|Default|GetGrid))
  (bind _tiledata (Default|GetTileData _grid Position))
  (Default|AddTileData _grid Position (Utilities|Struct|MakeST_TileData (.index _tiledata) (.transform _tiledata) (.position _tiledata) (.type _tiledata) (.states _tiledata) 0)))

(fn CastSpell
  (params (Range :type E_Spell%20Enum :default "NewEnumerator0") (AOE :type E_Spell%20Enum :default "NewEnumerator0") (Effect :type E_SpellEffectHandler%20Enum :default "NewEnumerator2") (Start%20Position :type Int%20Point%20Structure) (Range%20Position :type Int%20Point%20Structure) (AOE%20Positions :type Array%20of%20Int%20Point%20Structures) (Impact :type ST%20Spell%20Data%20Impact%20Structure))
  (bind _grid (Variables|Default|GetGrid))
  (bind (_bisoffensivespell _minmaxmodifier_hp _minmaxmodifier_mp _minmaxmodifier_ap) (Utilities|Struct|BreakST_SpellData_Impact Impact))
  (bind _tiledata (Default|GetTileData _grid Start%20Position))
  (bind _spelldata (CallFunction|GetSpellDatafromSpell Range))
  ;[0.03875 0.09734 0.1094] Caster Animation (Skeletal Mesh or not)
  (Utilities|IsValid (.unitontyle _tiledata)
    (:Is%20Valid
      (if (Default|CanCastSpell (.unitontyle _tiledata) _spelldata)
        (Default|UnitCastSpell (.unitontyle _tiledata) Range%20Position _spelldata)
        (else
          (return))))
    (:Is%20Not%20Valid
      _))
  ;[0.1302 0.1302 0.1302] Range Part
  (bind _output_get (LocalVariables|SetDataAssets (.Assets (Utilities|Struct|BreakST_SpellData (CallFunction|GetSpellDatafromSpell Range)))))
  (bind _returnvalue (Game|SpawnActorfromClass (.animation _output_get) (.transform (.TileData (Default|GetTileData (Variables|Default|GetGrid) Start%20Position))) "AlwaysSpawn" 0 0))
  (bind _output_get_2 (LocalVariables|SetRangeCast _returnvalue))
  (Utilities|IsValid _output_get_2
    (:Is%20Valid
      (Default|SetBasics _output_get_2 (Variables|Default|GetGrid) Start%20Position Range%20Position true))
    (:Is%20Not%20Valid
      (Development|PrintString "Combat System: No range cast. Melee?")))
  ;[0.1094 0.1094 0.1094] AOE Part
  (if (> (.x (Utilities|Array|Get(acopy) AOE%20Positions)) -999)
    (bind _output_get_3 (LocalVariables|SetDataAssets (.Assets (Utilities|Struct|BreakST_SpellData (CallFunction|GetSpellDatafromSpell AOE)))))
    (for _array_element AOE%20Positions
      (bind _returnvalue_2 (Game|SpawnActorfromClass (.animation _output_get_3) (.transform (.TileData (Default|GetTileData (Variables|Default|GetGrid) Range%20Position))) "AlwaysSpawn" 0 0))
      (Utilities|IsValid _returnvalue_2
        (:Is%20Valid
          (Default|SetBasics _returnvalue_2 (Variables|Default|GetGrid) Range%20Position _array_element false (LocalVariables|GetRangeCast)))
        (:Is%20Not%20Valid
          (Development|PrintString "Combat System: No AOE cast. Melee?")))))
  ;[0.1562 0 0] Affected Unit Animation (Skeletal Mesh or Not)
  (bind _output_get_4 (LocalVariables|SetTargetsPositions AOE%20Positions))
  (Utilities|Array|AddUnique _output_get_4 Range%20Position)
  (for _array_element_2 (LocalVariables|GetTargetsPositions)
    (Utilities|IsValid (.unitontyle (.TileData (Default|GetTileData (Variables|Default|GetGrid) _array_element_2)))
      (:Is%20Valid
        (bind _output_get_5 (LocalVariables|SetImpactResult (Utilities|Struct|MakeST_SpellData_Impact_Result (CallFunction|MinMaxRandom _minmaxmodifier_hp) (CallFunction|MinMaxRandom _minmaxmodifier_mp) (CallFunction|MinMaxRandom _minmaxmodifier_ap))))
        (Default|EventUnitHitbySpell (.unitontyle (.TileData (Default|GetTileData (Variables|Default|GetGrid) _array_element_2))) _output_get_5 (LocalVariables|GetRangeCast)))))
  ;[0 0.184 0] Spell Effect Handler part
  (if (Utilities|Enum|NotEqual(Enum) Effect "NewEnumerator2")
    (bind _out_row (CallFunction|GetSpellEffectDatafromSpellEffect Effect))
    (bind _returnvalue_3 (Game|SpawnActorfromClass (.Handler (Utilities|Struct|BreakST_SpellData_Effect _out_row)) (.transform (.TileData (Default|GetTileData (Variables|Default|GetGrid) Start%20Position))) "AlwaysSpawn" 0 0))
    (bind _output_get_6 (LocalVariables|SetSpellEffect _returnvalue_3))
    (Utilities|IsValid _output_get_6
      (:Is%20Valid
        (Default|SetBasicAttributes (LocalVariables|GetSpellEffect) Start%20Position Range%20Position AOE%20Positions)
        (Default|PlayEffect (LocalVariables|GetSpellEffect)))
      (:Is%20Not%20Valid
        (Development|PrintString "Combat System: Effect Error.")))))

(fn SetUnitTeamNumber
  (params (Unit :type BP%20Combatant%20Base%20Object%20Reference) (TeamNumber :type Byte))
  (Utilities|IsValid Unit
    (:Is%20Valid
      (Utilities|FlowControl|Sequence
        (:then_0
          ;[0.3594 0 0] Remove Unit from other team if already on a team
          (if (!= (Default|GetTeam Unit) 255)
            (bind _output_get (LocalVariables|SetUnit%20List (Utilities|Struct|BreakST_UnitSet (.Value (Utilities|Map|Find (Variables|Default|GetUnitTeams) (Default|GetTeam Unit))))))
            (Utilities|Set|Remove _output_get Unit)
            (if (> (Utilities|Set|Length (LocalVariables|GetUnit%20List)) 0)
              (Utilities|Map|Add (Variables|Default|GetUnitTeams) (Default|GetTeam Unit) (Utilities|Struct|MakeST_UnitSet (LocalVariables|GetUnit%20List)))
              (else
                (Utilities|Map|Remove (Variables|Default|GetUnitTeams) (Default|GetTeam Unit))))))
        (:then_1
          ;[0.03833 0.1222 0.8177] Added Unit on Mapping
          (if (!= TeamNumber 255)
            (bind _output_get_2 (LocalVariables|SetUnit%20List (Utilities|Struct|BreakST_UnitSet (.Value (Utilities|Map|Find (Variables|Default|GetUnitTeams) TeamNumber)))))
            (Utilities|Set|Add _output_get_2 Unit)
            (Utilities|Map|Add (Variables|Default|GetUnitTeams) TeamNumber (Utilities|Struct|MakeST_UnitSet (LocalVariables|GetUnit%20List)))))
        (:then_2
          ;[0.1874 0.7656 0.07178] Practical Effect on change team
          (Default|SetTeam Unit TeamNumber)
          (Default|CallOnUnitTeamChanged))))))

(fn GetUnitsonTeam
  (params (Team :type Byte%20%28by%20ref%29))
  (bind _unitteams (Variables|Default|GetUnitTeams))
  (bind (_value _returnvalue) (Utilities|Map|Find _unitteams Team))
  (return _returnvalue _value))

(fn CanStartCombat
  (bind _units (Variables|Default|GetUnits))
  (bind _unitteams (Variables|Default|GetUnitTeams))
  (bind _bisincombat (Variables|Default|GetbIsInCombat))
  (bind _returnvalue (Utilities|Array|Length _units))
  (bind _returnvalue_2 (Utilities|Map|Length _unitteams))
  (bind _returnvalue_3 (not _bisincombat))
  (bind _returnvalue_4 (>= _returnvalue_2 2))
  (bind _returnvalue_5 (>= _returnvalue 2))
  (return (Math|Boolean|ANDBoolean _returnvalue_5 _returnvalue_4 _returnvalue_3) _returnvalue_5 _returnvalue_4 _returnvalue_3))

(fn StartCombat
  (Combatant|ArrangeUnits)
  (Variables|Default|SetbIsInCombat true)
  (for _array_element (Variables|Default|GetUnits)
    (Utilities|IsValid _array_element
      (:Is%20Valid
        (Default|CombatStarted _array_element))
      (:Is%20Not%20Valid
        (Utilities|Array|RemoveItem (Variables|Default|GetUnits) _array_element))))
  (Default|CallOnCombatStarted)
  (Utilities|Array|Clear (Variables|Default|GetCurrentUnits))
  (Combatant|NextUnit))

(fn EndCombat
  (Variables|Default|SetbIsInCombat false)
  (Variables|Default|SetbIsFinishingCombat false)
  (for _array_element (Variables|Default|GetUnits)
    (Default|CombatEnded _array_element))
  (Default|CallOnCombatEnded)
  (Utilities|Array|Clear (Variables|Default|GetCurrentUnits)))

(fn NextUnit
  (if (Utilities|Array|IsEmpty (Variables|Default|GetCurrentUnits))
    _
    (else
      (for _array_element (Variables|Default|GetCurrentUnits)
        (Utilities|IsValid _array_element
          (:Is%20Valid
            (Default|TurnEnded _array_element)
            (Default|CallOnUnitTurnEnded _array_element))))
      (for _array_element_2 (Variables|Default|GetCurrentUnits)
        (if (> (Utilities|Array|FindItem (Variables|Default|GetUnits) _array_element_2) (LocalVariables|GetCurrentIndex))
          (LocalVariables|SetCurrentIndex (Utilities|Array|FindItem (Variables|Default|GetUnits) _array_element_2))))))
  (LocalVariables|SetCurrentIndex (+ (LocalVariables|GetCurrentIndex) 1) :!label _label)
  (while (not (Default|GetIsAlive (Utilities|Array|Get(acopy) (Variables|Default|GetUnits) (Math|Integer|%(Integer) (LocalVariables|GetCurrentIndex) (Utilities|Array|Length (Variables|Default|GetUnits))))))
    (goto _label))
  (Utilities|Array|Clear (Variables|Default|GetCurrentUnits))
  (Utilities|IsValid (Default|GetUnitAI (Utilities|Array|Get(acopy) (Variables|Default|GetUnits) (Math|Integer|%(Integer) (LocalVariables|GetCurrentIndex) (Utilities|Array|Length (Variables|Default|GetUnits)))))
    (:Is%20Valid
      (Default|TurnStarted (Utilities|Array|Get(acopy) (Variables|Default|GetUnits) (Math|Integer|%(Integer) (LocalVariables|GetCurrentIndex) (Utilities|Array|Length (Variables|Default|GetUnits)))))
      (Default|CallOnUnitTurnStarted (Utilities|Array|Get(acopy) (Variables|Default|GetUnits) (Math|Integer|%(Integer) (LocalVariables|GetCurrentIndex) (Utilities|Array|Length (Variables|Default|GetUnits)))))
      (Utilities|Array|Add (Variables|Default|GetCurrentUnits) (Utilities|Array|Get(acopy) (Variables|Default|GetUnits) (Math|Integer|%(Integer) (LocalVariables|GetCurrentIndex) (Utilities|Array|Length (Variables|Default|GetUnits))))))
    (:Is%20Not%20Valid
      (bind _unitset (Combatant|GetUnitsonTeam (Default|GetTeam (Utilities|Array|Get(acopy) (Variables|Default|GetUnits) (Math|Integer|%(Integer) (LocalVariables|GetCurrentIndex) (Utilities|Array|Length (Variables|Default|GetUnits)))))))
      (bind _result (Utilities|Set|ToArray (Utilities|Struct|BreakST_UnitSet _unitset)))
      (for _array_element_3 _result
        (Utilities|IsValid _array_element_3
          (:Is%20Valid
            (if (and (Default|GetIsAlive _array_element_3) (not (Utilities|IsValid (Default|GetUnitAI _array_element_3))))
              (Utilities|Array|AddUnique (Variables|Default|GetCurrentUnits) _array_element_3)
              (Default|TurnStarted _array_element_3)
              (Default|CallOnUnitTurnStarted _array_element_3))))))))

(fn SetLocationOfUnit
  (params (Position :type Int%20Point%20Structure) (Unit :type BP%20Combatant%20Base%20Object%20Reference))
  (bind _position (Default|GetPosition Unit))
  (bind _grid (Variables|Default|GetGrid))
  (bind (_success _tiledata) (Default|GetTileData _grid _position))
  (Utilities|IsValid Unit
    (:Is%20Valid
      (Default|GotoLocation Unit (Math|Vector|SelectVector (.location (.transform _tiledata)) "0.000000,0.000000,999999.000000" _success)))))

(fn HaveEnoughTeamstoContinue
  (bind _keys (Utilities|Map|Keys (Variables|Default|GetUnitTeams)))
  (for _array_element _keys
    (bind _output_get (LocalVariables|SetTeamVerify _array_element))
    (bind _result (Utilities|Set|ToArray (Utilities|Struct|BreakST_UnitSet (.Value (Utilities|Map|Find (Variables|Default|GetUnitTeams) _output_get)))))
    (bind _array_element_2 (Utilities|Array|ForEachLoopwithBreak _result :!label _label)
      (:LoopBody
        (Utilities|IsValid _array_element_2
          (:Is%20Valid
            (if (Default|GetIsAlive _array_element_2)
              (Utilities|Array|Add (LocalVariables|GetTeamsWithAliveMembers) (LocalVariables|GetTeamVerify))
              (goto _label Break)))))))
  (if (== (Utilities|Array|Length (LocalVariables|GetTeamsWithAliveMembers)) 1)
    (return false (Utilities|Array|Get(acopy) (LocalVariables|GetTeamsWithAliveMembers)))
    (else
      (return true 255))))

(fn HaveWinningTeam
  (params (WinningTeam :type Byte))
  (Variables|Default|SetbIsFinishingCombat true)
  (Default|CallOnCombatFinishing WinningTeam))

(fn GetUnits
  (return (Variables|Default|GetUnits)))

(fn SetUnitUseAI
  (params (Unit :type BP%20Combatant%20Base%20Object%20Reference) (bUseAI :type Boolean))
  (bind _aipawn (Default|GetUnitAI Unit))
  (if bUseAI
    (Utilities|IsValid (Default|GetUnitAI Unit)
      (:Is%20Not%20Valid
        (bind _returnvalue (Game|SpawnActorfromClass "/Game/TopDown/Blueprints/BP_AIPawn.BP_AIPawn_C" (Transformation|GetActorTransform Unit) "Undefined" 0 0))
        (Default|SetUnitAI Unit _returnvalue)
        (Default|SetCombatSystem _returnvalue self)
        (Default|SetControlledUnit _returnvalue Unit)))
    (else
      (Utilities|IsValid _aipawn
        (:Is%20Valid
          (Actor|DestroyActor _aipawn)
          (Default|SetUnitAI Unit))))))

(fn GetActiveTeams
  (bind _keys (Utilities|Map|Keys (Variables|Default|GetUnitTeams)))
  (return _keys))

(fn ArrangeUnits
  ;[0.1 0.1 0.1] Removing invalid units
  (bind _arrayelement (Utilities|Array|ReverseforEachLoop (Variables|Default|GetUnits))
    (:LoopBody
      (Utilities|IsValid _arrayelement
        (:Is%20Not%20Valid
          (Utilities|Array|RemoveItem (Variables|Default|GetUnits) _arrayelement))))
    (:Completed
      ;[0 0 0.1] Then, sorting if it have AI
      (for _array_element (Variables|Default|GetUnits)
        (Utilities|IsValid (Default|GetUnitAI _array_element)
          (:Is%20Valid
            (Utilities|Array|Add (LocalVariables|GetAIUnits) _array_element))
          (:Is%20Not%20Valid
            (Utilities|Array|Add (LocalVariables|GetNonAIUnits) _array_element))))
      ;[0.1 0 0] Then create a secondary array to order the teams number
      (LocalVariables|SetTeamsNumber (CallFunction|GetActiveTeams))
      (for (_ _array_index) (LocalVariables|GetTeamsNumber)
        (if (> _array_index 0)
          (for _index (range 0 (- _array_index 1))
            (if (> (Utilities|Array|Get(acopy) (LocalVariables|GetTeamsNumber) _index) (Utilities|Array|Get(acopy) (LocalVariables|GetTeamsNumber) _array_index))
              (Utilities|Array|Swap (LocalVariables|GetTeamsNumber) _index _array_index)))))
      ;[0 0.1 0] Last, sorting by team
      (Utilities|Array|Clear (Variables|Default|GetUnits))
      (for _array_element_2 (LocalVariables|GetTeamsNumber)
        (for _array_element_3 (LocalVariables|GetNonAIUnits)
          (if (== (Default|GetTeam _array_element_3) _array_element_2)
            (Utilities|Array|Add (Variables|Default|GetUnits) _array_element_3)))
        (for _array_element_4 (LocalVariables|GetAIUnits)
          (if (== (Default|GetTeam _array_element_4) _array_element_2)
            (Utilities|Array|Add (Variables|Default|GetUnits) _array_element_4)))))))

(fn GetIsinCombat
  (return (Variables|Default|GetbIsInCombat)))