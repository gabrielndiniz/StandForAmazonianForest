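; Grid combat action that previews a spell's range and casts it through BP_CombatSystem when the target tile is in range.
; Enabling casting stores the selected tile as origin and highlights valid tiles with instanced meshes; disabling clears them and reselects the origin.
; Range comes from pathfinding to maximum cost minus the minimum-cost area, then filtered by Line pattern and optional line-of-sight traces.
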(event EventBeginPlay
  (|CallParentFunction)
  (bind _returnvalue (Actor|GetActorOfClass "/Game/Combat/BP_CombatSystem.BP_CombatSystem_C" :!label _label))
  (bind _output_get (Variables|Default|SetCombatSystem _returnvalue))
  (Utilities|IsValid _output_get
    (:Is%20Not%20Valid
      (Utilities|FlowControl|Delay 1.0)
      (goto _label))))

(event Collision|EventActorBeginOverlap
  (params (OtherActor :type Actor%20Object%20Reference))
  (|CallParentFunction OtherActor) ; This node is disabled and will not be called.\nDrag off pins to build functionality.
)

(event EventTick
  (params (DeltaSeconds :type Float%20%28single-precision%29)))

(fn ConstructionScript
  (|CallParentFunction))

(fn GetIsCastingSpell
  (return (Variables|Default|GetbIsCastingSpell)))

(fn SetIsCastingSpell
  (params (bIsCastingSpell :type Boolean) (ActionManager :type BP%20Action%20Manager%20Object%20Reference))
  (bind _grid (Variables|Default|GetGrid))
  (Variables|Default|SetbIsCastingSpell bIsCastingSpell)
  (Variables|Default|SetAction%20Manager ActionManager)
  (if (Variables|Default|GetbIsCastingSpell)
    (CallFunction|ShowSpellRangePattern)
    (Variables|Default|SetOriginPosition (.SelectedPosition (Default|GetSelectedTile ActionManager)))
    (Default|SetShowReachables (Variables|/Game/TopDown/Blueprints/BP_ActionManager.BP_ActionManager_C|GetSelectTile ActionManager) false)
    (else
      (Components|InstancedStaticMesh|ClearInstances (Variables|Default|GetInstancedStaticMeshSpellRange))
      (if (> (.x (Variables|Default|GetOriginPosition)) -999)
        (Components|InstancedStaticMesh|ClearInstances (Variables|Default|GetInstancedStaticMeshSpellRange))
        (Default|SetTiletoHover ActionManager _grid (.Success (Default|GetTileData _grid (Variables|Default|GetOriginPosition))) (.location (.transform (.TileData (Default|GetTileData _grid (Variables|Default|GetOriginPosition))))))
        (Default|SetSelectedTile ActionManager)
        (Variables|Default|SetOriginPosition (Utilities|Struct|MakeIntPoint -999 -999))))))

(fn GetSpell
  (return (Variables|Default|GetSpellType)))

(fn SetSpellType
  (params (SpellType :type E_Spell%20Enum :default "NewEnumerator0"))
  (Variables|Default|SetSpellType SpellType))

(fn ExecuteAction
  (params (Position%201 :type Int%20Point%20Structure) (bHitResult :type Boolean) (Position%202 :type Int%20Point%20Structure))
  (bind (_success _tiledata1 _tiledata2) (|CallParentFunction Position%201 bHitResult Position%202))
  (Utilities|FlowControl|Sequence
    (:then_0
      (if (Math|Boolean|ANDBoolean (Variables|Default|GetbIsCastingSpell) (Utilities|Enum|NotEqual(Enum) (Variables|Default|GetSpellType) "NewEnumerator0") (Utilities|Array|ContainsItem (Variables|Default|GetPositionsInRange) Position%202))
        (Default|CastSpell (Variables|Default|GetCombatSystem) (Variables|Default|GetSpellType) Position%201 Position%202)))
    (:then_1
      (return _success _tiledata1 _tiledata2))))

(fn ShowSpellRangePattern
  (bind _positionsinrange (Variables|Default|GetPositionsInRange))
  (Components|InstancedStaticMesh|ClearInstances (Variables|Default|GetInstancedStaticMeshSpellRange))
  (bind _success (CallFunction|FindPositionsinRange))
  (if _success
    (if (> (.x (Utilities|Array|Get(acopy) (Variables|Default|GetPositionsInRange))) -999)
      (for _array_element (Variables|Default|GetPositionsInRange)
        (Components|InstancedStaticMesh|AddInstance (Variables|Default|GetInstancedStaticMeshSpellRange) (Math|Transform|MakeTransform (Math|Vector|MakeVector (.x (.location (.transform (.TileData (Default|GetTileData (Variables|Default|GetGrid) _array_element))))) (.y (.location (.transform (.TileData (Default|GetTileData (Variables|Default|GetGrid) _array_element))))) (+ (.z (.location (.transform (.TileData (Default|GetTileData (Variables|Default|GetGrid) _array_element))))) 4.0)) (.rotation (.transform (.TileData (Default|GetTileData (Variables|Default|GetGrid) _array_element)))) (.scale (.transform (.TileData (Default|GetTileData (Variables|Default|GetGrid) _array_element))))) true)))
    (else
      (Utilities|Array|Clear _positionsinrange)
      (Utilities|Array|Add _positionsinrange (Utilities|Struct|MakeIntPoint -999 -999)))))

(fn SetSpellRangePatternandRange
  (params (SpellRangePattern :type E_SpellRangePattern%20Enum :default "NewEnumerator0") (Spell%20Range%20Min%20Max :type Int%20Point%20Structure) (Spell%20Is%20Aerial :type Boolean) (Requires%20Line%20Of%20Sight :type Boolean) (DrawDebugLine :type Boolean) (Spell%20Data%20Cast%20Line%20Of%20Sight%20Height%20from%20Ground :type Float%20%28double-precision%29) (Spell%20Data%20Cast%20Line%20Of%20Sight%20Offset%20from%20Center :type Float%20%28double-precision%29))
  (Variables|Default|SetSpellDataCast (Utilities|Struct|MakeST_SpellData_Cast SpellRangePattern Spell%20Range%20Min%20Max Spell%20Is%20Aerial Requires%20Line%20Of%20Sight DrawDebugLine Spell%20Data%20Cast%20Line%20Of%20Sight%20Height%20from%20Ground Spell%20Data%20Cast%20Line%20Of%20Sight%20Offset%20from%20Center))
  (if (Variables|Default|GetbIsCastingSpell)
    (CallFunction|ShowSpellRangePattern)))

(fn FindPositionsinRange
  (bind _spelldatacast (Variables|Default|GetSpellDataCast))
  (bind _spelldatacast_2 (Variables|Default|GetSpellDataCast))
  (bind _action_manager (Variables|Default|GetAction%20Manager))
  (bind _action_manager_2 (Variables|Default|GetAction%20Manager))
  (bind _findpathtotitle (Variables|/Game/TopDown/Blueprints/BP_ActionManager.BP_ActionManager_C|GetFindPathToTitle _action_manager))
  (bind _findpathtotitle_2 (Variables|/Game/TopDown/Blueprints/BP_ActionManager.BP_ActionManager_C|GetFindPathToTitle _action_manager_2))
  (Utilities|FlowControl|Sequence
    (:then_0
      ;[0.07812 0.07812 0.07812] First, checking if function can continue.
      (if (Math|Boolean|ORBoolean (>= (.x (.rangeminmax _spelldatacast_2)) (.y (.rangeminmax _spelldatacast_2))) (< (.y (.rangeminmax _spelldatacast_2)) 0) (not (Utilities|IsValid (Variables|Default|GetAction%20Manager))) (Utilities|Enum|Equal(Enum) (.rangepattern (Variables|Default|GetSpellDataCast)) "NewEnumerator0") (Utilities|Enum|Equal(Enum) (Variables|Default|GetSpellType) "NewEnumerator0"))
        (return false)))
    (:then_1
      (Default|SetSelectedFlyingUnit (Variables|Default|GetAction%20Manager) (.bisaerial (Variables|Default|GetSpellDataCast)))
      ;[0.08854 0.08854 0.08854] Getting what is inside Range Y
      (Default|SetPathCost _findpathtotitle_2 (.y (.rangeminmax (Variables|Default|GetSpellDataCast))))
      (bind _path (Default|FindPath _findpathtotitle_2 (Variables|Default|GetOriginPosition) (Utilities|Struct|MakeIntPoint -999 -999) true true))
      (LocalVariables|SetRangeInY _path)
      (if (> (.x (.rangeminmax (Variables|Default|GetSpellDataCast))) 0)
        (Default|SetPathCost _findpathtotitle (.x (.rangeminmax (Variables|Default|GetSpellDataCast))))
        (bind _path_2 (Default|FindPath _findpathtotitle (Variables|Default|GetOriginPosition) (Utilities|Struct|MakeIntPoint -999 -999) true true))
        (LocalVariables|SetRangeInX _path_2)
        (for _array_element (LocalVariables|GetRangeInX)
          (if (Utilities|Array|ContainsItem (LocalVariables|GetRangeInY) _array_element)
            (Utilities|Array|RemoveItem (LocalVariables|GetRangeInY) _array_element)))))
    (:then_2
      ;[0.07812 0.07812 0.07812] Different Patterns Have Different Positions
      (switch Utilities|FlowControl|Switch|SwitchonE_SpellRangePattern (.rangepattern (Variables|Default|GetSpellDataCast))
        (:NewEnumerator1
          (bind (_arrayindex _arrayelement) (Utilities|Array|ReverseforEachLoop (LocalVariables|GetRangeInY))
            (:LoopBody
              (if (not (CallFunction|IsintheSameLine _arrayelement (Variables|Default|GetOriginPosition)))
                (Utilities|Array|RemoveIndex (LocalVariables|GetRangeInY) _arrayindex)))))))
    (:then_3
      (if (.brequirelineofsight _spelldatacast)
        (CallFunction|RemovePositionsWithoutLineOfSight (Variables|Default|GetOriginPosition) (.lineofsight_heightfromground _spelldatacast) (LocalVariables|GetRangeInY) (.blineofsight_drawdebugline _spelldatacast))))
    (:then_4
      (Utilities|Array|RemoveItem (LocalVariables|GetRangeInY) (Variables|Default|GetOriginPosition))
      (bind _output_get (Variables|Default|SetPositionsInRange (LocalVariables|GetRangeInY)))
      (return (> (Utilities|Array|Length _output_get) 0)))))

(fn HasLineOfSight
  (params (StartPosition :type Int%20Point%20Structure) (TargetPosition :type Int%20Point%20Structure) (UnitHeight :type Float%20%28double-precision%29) (OffSetFromCenter :type Float%20%28double-precision%29) (bDrawDebugLine :type Boolean))
  (LocalVariables|SetStartTile (.TileData (Default|GetTileData (Variables|Default|GetGrid) StartPosition)))
  (LocalVariables|SetTargetTile (.TileData (Default|GetTileData (Variables|Default|GetGrid) TargetPosition)))
  (LocalVariables|SetAdjustVector (Math|Vector|MakeVector 0.0 0.0 UnitHeight))
  (LocalVariables|SetStartLocation (+ (.location (.Transform (Utilities|Struct|BreakST_TileData (LocalVariables|GetStartTile)))) (LocalVariables|GetAdjustVector)))
  (LocalVariables|SetTargetLocation (+ (.location (.Transform (Utilities|Struct|BreakST_TileData (LocalVariables|GetTargetTile)))) (LocalVariables|GetAdjustVector)))
  (bind _returnvalue (Collision|LineTraceByChannel (LocalVariables|GetStartLocation) (LocalVariables|GetTargetLocation) "TraceTypeQuery6" false (Utilities|Array|MakeArray (.UnitOnTyle (Utilities|Struct|BreakST_TileData (LocalVariables|GetStartTile))) (.UnitOnTyle (Utilities|Struct|BreakST_TileData (LocalVariables|GetTargetTile)))) (Utilities|Enum|ByteToEnumEDrawDebugTrace (* (Math|Conversions|ToByte(Integer) bDrawDebugLine) 2))))
  (LocalVariables|SetBlocked _returnvalue)
  (if (and (!= OffSetFromCenter 0.0) (LocalVariables|GetBlocked))
    (for _array_element (Utilities|Array|MakeArray (+ (LocalVariables|GetTargetLocation) (Math|Vector|MakeVector OffSetFromCenter 0.0 0.0)) (+ (LocalVariables|GetTargetLocation) (Math|Vector|MakeVector (* OffSetFromCenter -1.0) 0.0 0.0)) (+ (LocalVariables|GetTargetLocation) (Math|Vector|MakeVector 0.0 OffSetFromCenter 0.0)) (+ (LocalVariables|GetTargetLocation) (Math|Vector|MakeVector 0.0 (* OffSetFromCenter -1.0) 0.0)))
      (bind _returnvalue_2 (Collision|LineTraceByChannel (LocalVariables|GetStartLocation) (LocalVariables|GetTargetLocation) "TraceTypeQuery6" false (Utilities|Array|MakeArray (.UnitOnTyle (Utilities|Struct|BreakST_TileData (LocalVariables|GetStartTile))) (.UnitOnTyle (Utilities|Struct|BreakST_TileData (LocalVariables|GetTargetTile)))) (Utilities|Enum|ByteToEnumEDrawDebugTrace (* (Math|Conversions|ToByte(Integer) bDrawDebugLine) 2))))
      (if (not _returnvalue_2)
        (return true)))
    (return false)
    (else
      (return (not (LocalVariables|GetBlocked))))))

(fn RemovePositionsWithoutLineOfSight
  (params (StartPosition :type Int%20Point%20Structure) (UnitHeight :type Float%20%28double-precision%29) (TargetPositions :type Array%20of%20Int%20Point%20Structures) (bDrawDebugLine :type Boolean))
  (bind (_arrayindex _arrayelement) (Utilities|Array|ReverseforEachLoop TargetPositions)
    (:LoopBody
      (if (not (CallFunction|HasLineOfSight StartPosition _arrayelement UnitHeight 0.0 bDrawDebugLine))
        (Utilities|Array|RemoveIndex TargetPositions _arrayindex)))))