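; BP_ハーベスター (Harvester) is an enemy Blueprint with a procedurally animated bladed-arm attack.
; BeginPlay calls InitiateData, then sets Joint, Wrist and Blades to their initial rotations.
; Attack and TestAttack share a DoOnce-gated Timeline that drives Joint and Blades yaw and Wrist roll.
; When the Timeline finishes, the parts snap back to their initial rotations and the gate resets, preventing overlapping swings.
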(event Custom|TestAttack
  (Utilities|FlowControl|DoOnce false :!label _label
    (:Completed
      (bind (_direction _jointrotation _wristrotation _bladesrotation) (Timeline|Timeline PlayFromStart)
        (:Update
          (Transformation|SetRelativeRotation (Variables|Default|GetJoint) (Math|Rotator|MakeRotator 0.0 0.0 _jointrotation) false false)
          (Transformation|SetRelativeRotation (Variables|Default|GetWrist) (Math|Rotator|MakeRotator _wristrotation 0.0 0.0) false false)
          (Transformation|SetRelativeRotation (Variables|Default|GetBlades) (Math|Rotator|MakeRotator 0.0 0.0 _bladesrotation) false false))
        (:Finished
          (Utilities|FlowControl|Sequence
            (:then_0
              (Transformation|SetRelativeRotation (Variables|Default|GetJoint) (Math|Rotator|MakeRotator 0.0 0.0 (Variables|Default|GetInitialJointRotation)) false false)
              (Transformation|SetRelativeRotation (Variables|Default|GetWrist) (Math|Rotator|MakeRotator (Variables|Default|GetInitialWristRotation) 0.0 0.0) false false)
              (Transformation|SetRelativeRotation (Variables|Default|GetBlades) (Math|Rotator|MakeRotator 0.0 0.0 (Variables|Default|GetInitialBladesRotation)) false false))
            (:then_1
              (goto _label Reset))))))))

(event EventBeginPlay
  (CallFunction|InitiateData)
  (Transformation|SetRelativeRotation (Variables|Default|GetJoint) (Math|Rotator|MakeRotator 0.0 0.0 (Variables|Default|GetInitialJointRotation)) false false)
  (Transformation|SetRelativeRotation (Variables|Default|GetWrist) (Math|Rotator|MakeRotator (Variables|Default|GetInitialWristRotation) 0.0 0.0) false false)
  (Transformation|SetRelativeRotation (Variables|Default|GetBlades) (Math|Rotator|MakeRotator 0.0 0.0 (Variables|Default|GetInitialBladesRotation)) false false))

(event EventAttack
  (params (Target%20Position :type Int%20Point%20Structure))
  (Utilities|FlowControl|DoOnce false :!label _label
    (:Completed
      (bind (_direction _jointrotation _wristrotation _bladesrotation) (Timeline|Timeline PlayFromStart)
        (:Update
          (Transformation|SetRelativeRotation (Variables|Default|GetJoint) (Math|Rotator|MakeRotator 0.0 0.0 _jointrotation) false false)
          (Transformation|SetRelativeRotation (Variables|Default|GetWrist) (Math|Rotator|MakeRotator _wristrotation 0.0 0.0) false false)
          (Transformation|SetRelativeRotation (Variables|Default|GetBlades) (Math|Rotator|MakeRotator 0.0 0.0 _bladesrotation) false false))
        (:Finished
          (Utilities|FlowControl|Sequence
            (:then_0
              (Transformation|SetRelativeRotation (Variables|Default|GetJoint) (Math|Rotator|MakeRotator 0.0 0.0 (Variables|Default|GetInitialJointRotation)) false false)
              (Transformation|SetRelativeRotation (Variables|Default|GetWrist) (Math|Rotator|MakeRotator (Variables|Default|GetInitialWristRotation) 0.0 0.0) false false)
              (Transformation|SetRelativeRotation (Variables|Default|GetBlades) (Math|Rotator|MakeRotator 0.0 0.0 (Variables|Default|GetInitialBladesRotation)) false false))
            (:then_1
              (goto _label Reset))))))))

(fn ConstructionScript
  (|CallParentFunction))