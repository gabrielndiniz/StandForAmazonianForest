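; Grid action that adds a unit to combat on a given tile or removes the one standing there.
; BeginPlay looks up BP_CombatSystem, retrying each second until it is valid.
; ExecuteAction calls the parent, then either spawns the selected unit type far above the world and registers it on a walkable tile, or removes and destroys the tile's occupant.
; It returns the parent's result regardless of the add or remove outcome.
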(event EventBeginPlay
  (|CallParentFunction)
  (bind _returnvalue (Actor|GetActorOfClass "/Game/Combat/BP_CombatSystem.BP_CombatSystem_C" :!label _label))
  (bind _output_get (Variables|Default|SetCombatSystem _returnvalue))
  (Utilities|IsValid _output_get
    (:Is%20Not%20Valid
      (Utilities|FlowControl|Delay 1.0)
      (goto _label))))

(event Collision|EventActorBeginOverlap
  (params (OtherActor :type Actor%20Object%20Reference))
  (|CallParentFunction OtherActor) ; This node is disabled and will not be called.\nDrag off pins to build functionality.
)

(event EventTick
  (params (DeltaSeconds :type Float%20%28single-precision%29)))

(fn ConstructionScript
  (|CallParentFunction))

(fn GetIsAddingUnit
  (return (Variables|Default|GetbIsAddingUnit)))

(fn SetIsAddingUnit
  (params (bIsAddingUnit :type Boolean))
  (Variables|Default|SetbIsAddingUnit bIsAddingUnit))

(fn GetUnitType
  (return (Variables|Default|GetUnitType)))

(fn SetUnitType
  (params (UnitType :type E_UnitType%20Enum :default "NewEnumerator0"))
  (Variables|Default|SetUnitType UnitType))

(fn ExecuteAction
  (params (Position%201 :type Int%20Point%20Structure) (bHitResult :type Boolean) (Position%202 :type Int%20Point%20Structure))
  (bind (_success _tiledata1 _tiledata2) (|CallParentFunction Position%201 bHitResult Position%202))
  (Utilities|FlowControl|Sequence
    (:then_0
      (if (Variables|Default|GetbIsAddingUnit)
        (CallFunction|AddUnit Position%201)
        (else
          (CallFunction|RemoveUnit Position%201))))
    (:then_1
      (return _success _tiledata1 _tiledata2))))

(fn AddUnit
  (params (Position%201 :type Int%20Point%20Structure))
  (if (Default|IsTileWalkable (Variables|Default|GetGrid) Position%201)
    (bind _returnvalue (Game|SpawnActorfromClass (Utilities|Select :Index (Variables|Default|GetUnitType) :NewEnumerator0 "/Game/Characters/Allies/Tocandira/BP_Tocandira.BP_Tocandira_C" :NewEnumerator1 "/Game/Characters/Allies/Caba/BP_Caba.BP_Caba_C" :NewEnumerator2 "/Game/Characters/Enemies/Blueprint/BP_Truck.BP_Truck_C" :NewEnumerator3 "/Game/Characters/Enemies/Blueprint/BP_ハーベスター.BP_ハーベスター_C" :NewEnumerator4 "/Game/Characters/Summon/BP_Içabebê.BP_Içabebê_C") (Math|Transform|MakeTransform "0.000000,0.000000,99999.000000" "0, 0, 0" "1.000000,1.000000,1.000000") "Undefined" 0 0))
    (bind _asbp_combatant_base (Utilities|Casting|CastToBP_Combatant_Base _returnvalue))
    (Default|AddUnitinCombat (Variables|Default|GetCombatSystem) _asbp_combatant_base Position%201)))

(fn RemoveUnit
  (params (Position%201 :type Int%20Point%20Structure))
  (bind _grid (Variables|Default|GetGrid))
  (bind (_success _tiledata) (Default|GetTileData _grid Position%201))
  (if (and _success (Utilities|IsValid (.unitontyle _tiledata)))
    (Default|RemoveUnitfromCombat (Variables|Default|GetCombatSystem) (.unitontyle _tiledata) true)))