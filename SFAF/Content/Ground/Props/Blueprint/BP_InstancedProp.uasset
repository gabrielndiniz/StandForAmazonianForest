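; BP_InstancedProp is a ground prop actor that displays its mesh snapped to the nearest point in a supplied grid.
; Its construction script clears the instanced mesh, then searches GridLocations for the point closest to the actor.
; It applies the configured mesh and material and adds one world-space instance there, offset by a spawn correction and the actor's height.
; No runtime event logic is active.
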(event EventBeginPlay)

(event Collision|EventActorBeginOverlap
  (params (OtherActor :type Actor%20Object%20Reference)))

(event EventTick
  (params (DeltaSeconds :type Float%20%28single-precision%29)))

(fn ConstructionScript
  (Components|InstancedStaticMesh|ClearInstances (Variables|Default|GetPropInstancedMesh))
  (CallFunction|SpawnMeshonGrid))

(fn SpawnMeshonGrid
  (bind _returnvalue (Transformation|GetActorLocation))
  (bind _propinstancedmesh (Variables|Default|GetPropInstancedMesh))
  (Utilities|FlowControl|Sequence
    (:then_0
      (Variables|Default|SetNewLocation (Utilities|Array|Get(acopy) (Variables|Default|GetGrid%20Locations))))
    (:then_1
      (for _array_element (Variables|Default|GetGrid%20Locations)
        (if (> (Math|Vector|Distance(Vector) (Variables|Default|GetNewLocation) _returnvalue) (Math|Vector|Distance(Vector) _array_element _returnvalue))
          (Variables|Default|SetNewLocation _array_element)))
      (Components|StaticMesh|SetStaticMesh _propinstancedmesh (Variables|Default|GetPropMesh))
      (Rendering|Material|SetMaterial _propinstancedmesh 0 (Variables|Default|GetPropMaterial))
      (Components|InstancedStaticMesh|AddInstance _propinstancedmesh (Math|Transform|MakeTransform (+ (Variables|Default|GetNewLocation) (Variables|Default|GetLocationSpawnCorrection) (Math|Vector|MakeVector 0.0 0.0 (.z (Transformation|GetActorLocation)))) "0, 0, 0" "1.000000,1.000000,1.000000") true))))