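; BP_Truck is an enemy truck Blueprint with a TestAttack event that drives its static mesh through a timed lunge.
; BeginPlay caches the mesh's relative location as the origin.
; TestAttack plays a timeline whose float curve scales the actor's forward vector and Velocity, applying the offset as an unswept relative location.
; When the timeline finishes, the mesh snaps back to its cached location.
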(event Custom|TestAttack
  (bind _floatcurve (Timeline|Timeline PlayFromStart)
    (:Update
      (Transformation|SetRelativeLocation (Variables|Default|GetStaticMesh) (+ (* _floatcurve (Transformation|GetActorForwardVector) (Variables|Default|GetVelocity)) (Variables|Default|GetInitial%20Location)) false false))
    (:Finished
      (Transformation|SetRelativeLocation (Variables|Default|GetStaticMesh) (Variables|Default|GetInitial%20Location) false false))))

(event EventBeginPlay
  (Variables|Default|SetInitial%20Location (Variables|/Script/Engine.SceneComponent|GetRelativeLocation (Variables|Default|GetStaticMesh))))

(event Collision|EventActorBeginOverlap
  (params (OtherActor :type Actor%20Object%20Reference)))

(event EventTick
  (params (DeltaSeconds :type Float%20%28single-precision%29)))

(fn ConstructionScript
  (|CallParentFunction))