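; Spell animation actor that plays animated shapes travelling from an origin grid tile to target tiles.
; Shortly after BeginPlay it spawns a BP_AnimatedShape at the origin tile for each target and passes it both tile transforms.
; Completed shapes are collected until their count matches the targets, then it broadcasts OnSpellAnimationCompleted and destroys itself after a short delay.
; SetBasics supplies the grid and origin, and appends a target.
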(event Custom|Event_PlaySpellAnimation
  (for _array_element (Variables|Default|GetTargetPositions)
    (Variables|Default|SetCurrentTargetPosition _array_element)
    (bind _returnvalue (Game|SpawnActorfromClass "/Game/Combat/Spells/Components/BP_AnimatedShape.BP_AnimatedShape_C" (.transform (.TileData (Default|GetTileData (Variables|Default|GetGrid) (Variables|Default|GetOriginPosition)))) "AlwaysSpawn" 0 0))
    (EventDispatchers|BindEventtoOnShapeAnimationCompleted _returnvalue (delegate Custom|OnShapeAnimationCompleted))
    (Default|SetTransforms _returnvalue (.transform (.TileData (Default|GetTileData (Variables|Default|GetGrid) (Variables|Default|GetOriginPosition)))) (.transform (.TileData (Default|GetTileData (Variables|Default|GetGrid) (Variables|Default|GetCurrentTargetPosition)))))))

(event Custom|CompletedSpellAnimation
  (if (== (Utilities|Array|Length (Variables|Default|GetTargetPositions)) (Utilities|Array|Length (Variables|Default|GetAnimated%20Shapes)))
    (Default|CallOnSpellAnimationCompleted self)
    (Utilities|FlowControl|Delay 0.2)
    (Actor|DestroyActor)))

(event Custom|OnShapeAnimationCompleted
  (params (AnimatedShape :type BP%20Animated%20Shape%20Object%20Reference))
  (Utilities|Array|AddUnique (Variables|Default|GetAnimated%20Shapes) AnimatedShape)
  (CallFunction|CompletedSpellAnimation))

(event EventBeginPlay
  (Utilities|FlowControl|Delay 0.2)
  (CallFunction|EventPlaySpellAnimation))

(fn ConstructionScript)

(fn SetBasics
  (params (Grid :type BP%20Grid%20Object%20Reference) (OriginPosition :type Int%20Point%20Structure) (TargetPosition :type Int%20Point%20Structure))
  (Variables|Default|SetGrid Grid)
  (Variables|Default|SetOriginPosition OriginPosition)
  (Utilities|Array|Add (Variables|Default|GetTargetPositions) TargetPosition))