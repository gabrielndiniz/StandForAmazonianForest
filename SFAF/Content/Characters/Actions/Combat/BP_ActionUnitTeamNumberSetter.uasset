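; Grid action that assigns a stored team number to the unit standing on the targeted tile.
; On BeginPlay it looks up the BP_CombatSystem actor, retrying every second until found.
; ExecuteAction runs the parent action, reads the tile at the first position and, if a unit occupies it, passes that unit and TeamNumber to the combat system.
; SetTeamNumber changes the number to apply.
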(event EventBeginPlay
  (|CallParentFunction)
  (bind _returnvalue (Actor|GetActorOfClass "/Game/Combat/BP_CombatSystem.BP_CombatSystem_C" :!label _label))
  (bind _output_get (Variables|Default|SetCombatSystem _returnvalue))
  (Utilities|IsValid _output_get
    (:Is%20Not%20Valid
      (Utilities|FlowControl|Delay 1.0)
      (goto _label))))

(event Collision|EventActorBeginOverlap
  (params (OtherActor :type Actor%20Object%20Reference))
  (|CallParentFunction OtherActor) ; This node is disabled and will not be called.\nDrag off pins to build functionality.
)

(event EventTick
  (params (DeltaSeconds :type Float%20%28single-precision%29)))

(fn ConstructionScript
  (|CallParentFunction))

(fn ExecuteAction
  (params (Position%201 :type Int%20Point%20Structure) (bHitResult :type Boolean) (Position%202 :type Int%20Point%20Structure))
  (bind _grid (Variables|Default|GetGrid))
  (bind (_success _tiledata) (Default|GetTileData _grid Position%201))
  (bind _unitontyle (Utilities|Struct|BreakST_TileData _tiledata))
  (bind (_success_2 _tiledata1 _tiledata2) (|CallParentFunction Position%201 bHitResult Position%202))
  (Utilities|FlowControl|Sequence
    (:then_0
      (if _success
        (Utilities|IsValid _unitontyle
          (:Is%20Valid
            (Default|SetUnitTeamNumber (Variables|Default|GetCombatSystem) _unitontyle (Variables|Default|GetTeamNumber))))))
    (:then_1
      (return _success_2 _tiledata1 _tiledata2))))

(fn SetTeamNumber
  (params (TeamNumber :type Byte))
  (Variables|Default|SetTeamNumber TeamNumber))