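; Grid modifier actor that carries a tile type (None, Normal or Obstacle), exposed through GetTileType.
; The construction script takes the solid mesh from the grid data component's shape, colors it by type and applies brightness parameters for emission and opacity.
; It also sets the mesh to overlap on a custom collision channel and keeps it visible in game, with no active event graph logic.
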(event EventBeginPlay)

(event Collision|EventActorBeginOverlap
  (params (OtherActor :type Actor%20Object%20Reference)))

(event EventTick
  (params (DeltaSeconds :type Float%20%28single-precision%29)))

(fn ConstructionScript
  (bind _staticmesh (Variables|Default|GetStaticMesh))
  (Components|StaticMesh|SetStaticMesh _staticmesh (.Solid (Default|GetShapeData (Variables|Default|GetBP_GridDataComponent))))
  (Rendering|Material|SetVectorParameterValueonMaterials _staticmesh "Color" (Math|Conversions|ToVector(LinearColor) (Utilities|Select :Index (Variables|Default|GetType) :NewEnumerator0 "(R=0.000000,G=1.000000,B=0.000000,A=1.000000)" :NewEnumerator1 "(R=0.000000,G=0.000000,B=0.000000,A=1.000000)" :NewEnumerator2 "(R=1.000000,G=0.000000,B=0.000000,A=1.000000)")))
  ;[1 1 1] This segment will decide if there will be color or not on the StaticMesh. It will bright from inside, not from outside.
  (Rendering|Material|SetScalarParameterValueonMaterials _staticmesh "MultiplierForEmissionAndOpacity" (Variables|Default|GetBrightMultiply))
  (Rendering|Material|SetScalarParameterValueonMaterials _staticmesh "AddAfterMultiplier" (Variables|Default|GetBrightAdder))
  (Collision|SetCollisionResponsetoChannel (Variables|Default|GetStaticMesh) "ECC_GameTraceChannel3" "ECR_Overlap")
  (Development|SetHiddeninGame (Variables|Default|GetStaticMesh) false false))

(fn GetTileType
  (return (Variables|Default|GetType)))