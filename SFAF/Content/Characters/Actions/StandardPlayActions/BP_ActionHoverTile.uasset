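; Player action actor that highlights the grid tile being hovered and places a hover plane on it.
; ExecuteAction runs the parent action, then moves the plane to the returned tile location, or hides it on failure.
; SetTileStatus tracks the hovered index, moving the hover state between Grid tiles and applying another state when the hit is lost.
; It checks the selected tile through BP_ActionSelectTile, found shortly after BeginPlay.
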(event EventBeginPlay
  (|CallParentFunction)
  (Utilities|FlowControl|Delay 0.2)
  (bind _returnvalue (Actor|GetActorOfClass "/Game/Characters/Actions/StandardPlayActions/BP_ActionSelectTile.BP_ActionSelectTile_C"))
  (Variables|Default|SetSelect _returnvalue))

(event Collision|EventActorBeginOverlap
  (params (OtherActor :type Actor%20Object%20Reference))
  (|CallParentFunction OtherActor) ; This node is disabled and will not be called.\nDrag off pins to build functionality.
)

(event EventTick
  (params (DeltaSeconds :type Float%20%28single-precision%29))
  (|CallParentFunction DeltaSeconds) ; This node is disabled and will not be called.\nDrag off pins to build functionality.
)

(fn ConstructionScript
  (|CallParentFunction))

(fn SetHoverPlaneLocation
  (params (NewLocation :type Vector) (bHide :type Boolean))
  (bind _hoverplane (Variables|Default|GetHoverPlane))
  (if (Utilities|Operators|NotEqual(!=) NewLocation (Transformation|GetWorldLocation (Variables|Default|GetHoverPlane)) 0.01)
    (if bHide
      (Rendering|SetVisibility _hoverplane false false)
      (else
        (Transformation|SetWorldLocation _hoverplane NewLocation false false)
        (if (not (Rendering|IsVisible (Variables|Default|GetHoverPlane)))
          (Rendering|SetVisibility (Variables|Default|GetHoverPlane) true true))))))

(fn ExecuteAction
  (params (Index :type Integer) (bHitResult :type Boolean))
  (bind (_success _tiledata) (|CallParentFunction Index bHitResult))
  (LocalVariables|SetContinue _success)
  (CallFunction|SetTileStatus bHitResult Index)
  (if (LocalVariables|GetContinue)
    (LocalVariables|SetData _tiledata)
    (CallFunction|SetHoverPlaneLocation (.location (.transform (LocalVariables|GetData))) false)
    (else
      (CallFunction|SetHoverPlaneLocation "0.000000,0.000000,9999.000000" true)
      (return (LocalVariables|GetContinue) (LocalVariables|GetData)))))

(fn SetTileStatus
  (params (bHitResult :type Boolean) (Index :type Integer))
  (if bHitResult
    (LocalVariables|SetCurrentIndex Index)
    (if (!= (Default|GetSelectedTile (Variables|Default|GetSelect)) (LocalVariables|GetCurrentIndex))
      (if (!= (LocalVariables|GetCurrentIndex) (Variables|Default|GetHoveredGridIndex))
        (Default|RemoveStateTile (Variables|Default|GetGrid) (Variables|Default|GetHoveredGridIndex) "NewEnumerator1")
        (Variables|Default|SetHoveredGridIndex (LocalVariables|GetCurrentIndex))
        (Default|AddStateTile (Variables|Default|GetGrid) (LocalVariables|GetCurrentIndex) "NewEnumerator1"))
      (elif (!= (Default|GetSelectedTile (Variables|Default|GetSelect)) (Variables|Default|GetHoveredGridIndex))
        (Default|RemoveStateTile (Variables|Default|GetGrid) (Variables|Default|GetHoveredGridIndex) "NewEnumerator1")
        (bind _output_get (Variables|Default|SetHoveredGridIndex (Default|GetSelectedTile (Variables|Default|GetSelect))))
        (Default|AddStateTile (Variables|Default|GetGrid) _output_get "NewEnumerator1")))
    (elif (!= (Variables|Default|GetHoveredGridIndex) -1)
      (Default|AddStateTile (Variables|Default|GetGrid) (Variables|Default|GetHoveredGridIndex) "NewEnumerator0")
      (Variables|Default|SetHoveredGridIndex -1))))