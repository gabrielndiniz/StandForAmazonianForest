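; Grid action that finds a walkable tile path between two positions, flags its tiles on the grid and optionally shows it with instanced meshes.
; FindPath runs an A*-style search, discovering neighbors from ShowTileNeighbor into a cost-sorted list with Chebyshev distance estimates.
; It expands the discovered tile GetNearestTileFromTarget picks, rather than the list's cheapest.
; GeneratePath backtracks previous positions, capped by a grid-size limit against infinite loops.
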(event EventBeginPlay
  (bind _grid (Variables|Default|GetGrid))
  (bind _gridlastposition (Default|GetGridLastPosition _grid))
  (|CallParentFunction)
  (Utilities|FlowControl|Delay 0.8)
  ;[0.04688 0.04688 0.04688] To reduce chance of infinite loop.
  (Variables|Default|SetMaxExpectedInteractions (+ (.x _gridlastposition) (.y _gridlastposition))))

(event Collision|EventActorBeginOverlap
  (params (OtherActor :type Actor%20Object%20Reference))
  (|CallParentFunction OtherActor) ; This node is disabled and will not be called.\nDrag off pins to build functionality.
)

(event EventTick
  (params (DeltaSeconds :type Float%20%28single-precision%29))
  (|CallParentFunction DeltaSeconds) ; This node is disabled and will not be called.\nDrag off pins to build functionality.
)

(fn ConstructionScript
  (|CallParentFunction))

(fn ExecuteAction
  (params (Position%201 :type Int%20Point%20Structure) (bHitResult :type Boolean) (Position%202 :type Int%20Point%20Structure))
  (bind (_success _tiledata1 _tiledata2) (|CallParentFunction Position%201 bHitResult Position%202))
  (Utilities|FlowControl|Sequence
    (:then_0
      (if (!= Position%201 (Variables|Default|GetCurrentPositon))
        (CallFunction|ClearGeneratedData)
        (if bHitResult
          (bind _path (CallFunction|FindPath Position%201 Position%202))
          (bind _output_get (Variables|Default|SetPath _path))
          (for _array_element _output_get
            (Default|AddStateTile (Variables|Default|GetGrid) _array_element "NewEnumerator4")
            (CallFunction|ShowPath)))))
    (:then_1
      (return _success _tiledata1 _tiledata2))))

(fn SetShowTileNeighbor
  (params (ShowTileNeighbor :type BP%20Action%20Show%20Tile%20Neighbor%20Object%20Reference))
  (Variables|Default|SetShowTileNeighbor ShowTileNeighbor))

(fn SetShowPath
  (params (bShowPath :type Boolean))
  (Variables|Default|SetbShowPath bShowPath))

(fn ShowPath
  (Components|InstancedStaticMesh|ClearInstances (Variables|Default|GetInstancedStaticMesh))
  (if (Variables|Default|GetbShowPath)
    (for _array_element (Variables|Default|GetPath)
      (Components|InstancedStaticMesh|AddInstance (Variables|Default|GetInstancedStaticMesh) (.transform (.TileData (Default|GetTileData (Variables|Default|GetGrid) _array_element))) true))))

(fn FindPath
  (params (Start :type Int%20Point%20Structure) (Target :type Int%20Point%20Structure))
  (Utilities|FlowControl|Sequence
    (:then_0
      (CallFunction|ClearGeneratedData))
    (:then_1
      (Variables|Default|SetStartPosition Start)
      (Variables|Default|SetTargetPosition Target)
      (bind _bisvalid (CallFunction|IsInputDataValid))
      (if _bisvalid
        (bind _mincost (CallFunction|GetMinimumCostBetweenTwoTiles Start Target))
        (CallFunction|DiscoverTile (Utilities|Struct|MakeST_PathfindingData Start 1 0 _mincost "(X=999,Y=999)"))
        (while (> (Utilities|Array|Length (Variables|Default|GetDiscoveredTilePosition)) 0)
          (bind _foundtargettile (CallFunction|AnalyseNextDiscoveredTile))
          (if _foundtargettile
            (bind _path (CallFunction|GeneratePath))
            (return _path true)))))
    (:then_2
      (return (LocalVariables|GetPositions) false))))

(fn IsInputDataValid
  (return (Math|Boolean|ANDBoolean (Default|IsTileWalkable (Variables|Default|GetGrid) (Variables|Default|GetStartPosition)) (Default|IsTileWalkable (Variables|Default|GetGrid) (Variables|Default|GetTargetPosition)) (!= (Variables|Default|GetStartPosition) (Variables|Default|GetTargetPosition)))))

(fn DiscoverTile
  (params (TilePathData :type ST%20Pathfinding%20Data%20Structure))
  (Utilities|Map|Add (Variables|Default|GetPathfindingData) (.Position (Utilities|Struct|BreakST_PathfindingData TilePathData)) TilePathData)
  (CallFunction|InsertTileinDiscoveredArray TilePathData))

(fn GetMinimumCostBetweenTwoTiles
  (params (Position1 :type Int%20Point%20Structure) (Position2 :type Int%20Point%20Structure))
  (bind _returnvalue (- Position1 Position2))
  ;[0.05208 0.05208 0.05208] Modifying from the video. https://www.youtube.com/watch?v=xakl29fupCA&list=PLBLmKCAjA25CKFIvmaA8y3tsX_URgkX4O&index=30
  (return (Math|Integer|Max(Integer) (Math|Integer|Absolute(Integer) (.x _returnvalue)) (Math|Integer|Absolute(Integer) (.y _returnvalue)))))

(fn AnalyseNextDiscoveredTile
  (Utilities|FlowControl|Sequence
    (:then_0
      (bind _tilepathdata (CallFunction|PullCheapestTileOutOfDiscoveredList))
      (bind _output_get (Variables|Default|SetCurrentDiscoveredTile _tilepathdata))
      (bind _neighborpositions (Default|GetTileNeighbors (Variables|Default|GetShowTileNeighbor) (.position _output_get)))
      (Variables|Default|SetCurrentNeighbors _neighborpositions)
      (while (> (Utilities|Array|Length (Variables|Default|GetCurrentNeighbors)) 0)
        (bind _bistargettile (CallFunction|DiscoverNextNeighbor))
        (if _bistargettile
          (return true))))
    (:then_1
      (return false))))

(fn GeneratePath
  (LocalVariables|SetCurrent (Variables|Default|GetTargetPosition))
  (while (and (!= (LocalVariables|GetCurrent) (Variables|Default|GetStartPosition)) (< (LocalVariables|GetCount) (Variables|Default|GetMaxExpectedInteractions)))
    (Utilities|Array|Add (LocalVariables|GetInvertedPath) (LocalVariables|GetCurrent))
    (LocalVariables|SetCurrent (.previousposition (.Value (Utilities|Map|Find (Variables|Default|GetPathfindingData) (LocalVariables|GetCurrent)))))
    (LocalVariables|SetCount (+ (LocalVariables|GetCount) 1)))
  (bind _arrayelement (Utilities|Array|ReverseforEachLoop (LocalVariables|GetInvertedPath))
    (:LoopBody
      (Utilities|Array|Add (LocalVariables|GetResult) _arrayelement))
    (:Completed
      (return (LocalVariables|GetResult)))))

(fn PullCheapestTileOutOfDiscoveredList
  (bind _index (Default|GetNearestTilefromTarget (Variables|Default|GetGrid) (Variables|Default|GetDiscoveredTilePosition) (Variables|Default|GetTargetPosition)))
  (LocalVariables|SetIndexToUse _index)
  (LocalVariables|SetTilePosition (Utilities|Array|Get(acopy) (Variables|Default|GetDiscoveredTilePosition) (LocalVariables|GetIndexToUse)))
  (Utilities|Array|RemoveIndex (Variables|Default|GetDiscoveredTileSortingCosts) (LocalVariables|GetIndexToUse))
  (Utilities|Array|RemoveIndex (Variables|Default|GetDiscoveredTilePosition) (LocalVariables|GetIndexToUse))
  (Utilities|Array|Add (Variables|Default|GetAnalysedTilePositions) (LocalVariables|GetTilePosition))
  (return (.Value (Utilities|Map|Find (Variables|Default|GetPathfindingData) (LocalVariables|GetTilePosition)))))

(fn DiscoverNextNeighbor
  (Utilities|FlowControl|Sequence
    (:then_0
      (Variables|Default|SetCurrentNeighbor (Utilities|Array|Get(acopy) (Variables|Default|GetCurrentNeighbors)))
      (Utilities|Array|RemoveIndex (Variables|Default|GetCurrentNeighbors))
      (if (not (Utilities|Array|ContainsItem (Variables|Default|GetAnalysedTilePositions) (.position (Variables|Default|GetCurrentNeighbor))))
        (LocalVariables|SetCostFromStart (+ (.costfromstart (Variables|Default|GetCurrentDiscoveredTile)) (.minimumcosttotarget (Variables|Default|GetCurrentNeighbor))))
        (bind _output_get (LocalVariables|SetIndexDiscovered (Utilities|Array|FindItem (Variables|Default|GetDiscoveredTilePosition) (.position (Variables|Default|GetCurrentNeighbor)))))
        (if (== _output_get -1)
          (bind _mincost (CallFunction|GetMinimumCostBetweenTwoTiles (.Position (Utilities|Struct|BreakST_PathfindingData (Variables|Default|GetCurrentNeighbor))) (Variables|Default|GetTargetPosition) :!label _label))
          (CallFunction|DiscoverTile (Utilities|Struct|MakeST_PathfindingData (.Position (Utilities|Struct|BreakST_PathfindingData (Variables|Default|GetCurrentNeighbor))) (.CostToEnterTile (Utilities|Struct|BreakST_PathfindingData (Variables|Default|GetCurrentNeighbor))) (LocalVariables|GetCostFromStart) _mincost (.position (Variables|Default|GetCurrentDiscoveredTile))))
          (if (Class|KismetMathLibrary|EqualIntPointIntPoint (.Position (Utilities|Struct|BreakST_PathfindingData (Variables|Default|GetCurrentNeighbor))) (Variables|Default|GetTargetPosition))
            (return true))
          (else
            (bind _output_get_2 (Variables|Default|SetCurrentNeighbor (.Value (Utilities|Map|Find (Variables|Default|GetPathfindingData) (.position (Variables|Default|GetCurrentNeighbor))))))
            (if (< (LocalVariables|GetCostFromStart) (.costfromstart _output_get_2))
              (Utilities|Array|RemoveIndex (Variables|Default|GetDiscoveredTilePosition) (LocalVariables|GetIndexDiscovered))
              (Utilities|Array|RemoveIndex (Variables|Default|GetDiscoveredTileSortingCosts) (LocalVariables|GetIndexDiscovered))
              (goto _label))))))
    (:then_1
      (return false))))

(fn InsertTileinDiscoveredArray
  (params (TileData :type ST%20Pathfinding%20Data%20Structure))
  (bind _discoveredtilesortingcosts (Variables|Default|GetDiscoveredTileSortingCosts))
  (LocalVariables|SetSortingCost (+ (.costfromstart TileData) (.minimumcosttotarget TileData)))
  (if (== (Utilities|Array|Length (Variables|Default|GetDiscoveredTileSortingCosts)) 0)
    (Utilities|Array|Add (Variables|Default|GetDiscoveredTileSortingCosts) (LocalVariables|GetSortingCost) :!label _label)
    (Utilities|Array|Add (Variables|Default|GetDiscoveredTilePosition) (.position TileData))
    (elif (>= (LocalVariables|GetSortingCost) (Utilities|Array|Get(acopy) _discoveredtilesortingcosts (Utilities|Array|LastIndex _discoveredtilesortingcosts)))
      (goto _label)
      (else
        (bind (_array_element _array_index) (Utilities|Array|ForEachLoopwithBreak (Variables|Default|GetDiscoveredTileSortingCosts) :!label _label_2)
          (:LoopBody
            (LocalVariables|SetIndexToConsider _array_index)
            (if (>= _array_element (LocalVariables|GetSortingCost))
              (Utilities|Array|Insert (Variables|Default|GetDiscoveredTileSortingCosts) (LocalVariables|GetSortingCost) (LocalVariables|GetIndexToConsider))
              (Utilities|Array|Insert (Variables|Default|GetDiscoveredTilePosition) (.position TileData) (LocalVariables|GetIndexToConsider))
              (goto _label_2 Break))))))))

(fn ClearGeneratedData
  (Utilities|Array|Clear (Variables|Default|GetDiscoveredTilePosition))
  (Utilities|Array|Clear (Variables|Default|GetDiscoveredTileSortingCosts))
  (Utilities|Array|Clear (Variables|Default|GetDiscoveredTilePosition))
  (Utilities|Array|Clear (Variables|Default|GetAnalysedTilePositions))
  (for _array_element (Variables|Default|GetPath)
    (Default|RemoveStateTile (Variables|Default|GetGrid) _array_element "NewEnumerator4"))
  (Utilities|Array|Clear (Variables|Default|GetPath))
  (Components|InstancedStaticMesh|ClearInstances (Variables|Default|GetInstancedStaticMesh)))