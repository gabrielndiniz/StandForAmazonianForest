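; BP_MeleeFight is an animated shape for combat spells that plays a melee hit effect between an origin and a target.
; When its transforms are set, it points the NSHit effect's Direction along the normalized vector from target to origin and activates it with a reset.
; It then passes both transforms to the parent implementation, while its AnimationComplete override is empty.
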(fn ConstructionScript
  (|CallParentFunction))

(fn AnimationComplete)

(fn SetTransforms
  (params (OriginTransform :type Transform) (TargetTransform :type Transform) (Position :type Int%20Point%20Structure))
  (bind _ns_hit (Variables|Default|GetNS_Hit))
  (Utilities|FlowControl|Sequence
    (:then_0
      (Effects|Components|ParticleSystem|SetVectorParameter _ns_hit "Direction" (Math|Vector|Normalize (- (.location OriginTransform) (.location TargetTransform))))
      (Components|Activation|Activate _ns_hit true))
    (:then_1
      (|CallParentFunction OriginTransform TargetTransform ""))))