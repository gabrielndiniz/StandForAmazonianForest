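; BP_Grid is a terrain grid actor that builds a hexagonal tile field from instanced static meshes in its construction script.
; SpawnGrid snaps the origin, optionally centred, then lays two offset tile lattices with an 8/7 Y correction for hex geometry.
; The Color enum selects mesh and material from DT_GridShapeData.
; With SpawnOnEnvironment, sphere traces place tiles only where ground is hit, snapping their height to the grid.
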(event EventBeginPlay)

(event Collision|EventActorBeginOverlap
  (params (OtherActor :type Actor%20Object%20Reference)))

(event EventTick
  (params (DeltaSeconds :type Float%20%28single-precision%29)))

(fn ConstructionScript
  (CallFunction|SpawnGrid (Transformation|GetActorLocation) (Variables|Default|GetGrid%20Tile%20Size) (Variables|Default|GetGrid%20Tile%20Count) (Variables|Default|GetColor) (Variables|Default|GetbSpawn%20Around%20Given%20Location) (Variables|Default|GetbSpawn%20on%20Environment)))

(fn SpawnGrid
  (params (Initial%20Spawn%20Location :type Vector) (TileSize :type Vector) (TileCount :type Int%20Point%20Structure) (Color :type E_GridShape%20Enum :default "NewEnumerator0") (bSpawnAroundLocation :type Boolean) (bSpawnOnEnvironment :type Boolean))
  (bind (_meshsize _mesh _material) (CallFunction|GetCurrentShapeData))
  (bind _instancedstaticmesh (Variables|Default|GetInstancedStaticMesh))
  (CallFunction|DestroyGrid)
  (if (not (Utilities|Enum|Equal(Enum) Color "NewEnumerator0"))
    (CallFunction|SetCurrentShapeData Initial%20Spawn%20Location TileSize TileCount Color bSpawnAroundLocation bSpawnOnEnvironment)
    (Components|StaticMesh|SetStaticMesh _instancedstaticmesh _mesh)
    (Rendering|Material|SetMaterial _instancedstaticmesh 0 _material)
    (bind _newparam (CallFunction|SnapInitialLocation))
    (Variables|Default|SetGridBottomLeftCurrentLocation _newparam)
    (for _index (range 0 (- (.x (Variables|Default|GetGrid%20Tile%20Count)) 1))
      (LocalVariables|SetXDirection _index)
      (for _index_2 (range 0 (- (.y (Variables|Default|GetGrid%20Tile%20Count)) 1))
        (LocalVariables|SetYDirection (+ _index_2 1))
        (Utilities|FlowControl|Sequence
          (:then_0
            ;[1 1 1] Spawn Mesh on Even Collums
            (bind _output_get (LocalVariables|SetTileTransform (Math|Transform|MakeTransform (+ (Variables|Default|GetGridBottomLeftCurrentLocation) (* (Variables|Default|GetGrid%20Tile%20Size) (Math|Vector|MakeVector (Math|Conversions|ToFloat(Integer) (LocalVariables|GetXDirection)) (/ (* (Math|Conversions|ToFloat(Integer) (LocalVariables|GetYDirection)) 8.0) 7.0) 0.0))) "0, 0, 0" (/ (Variables|Default|GetGrid%20Tile%20Size) (.MeshSize (CallFunction|GetCurrentShapeData))))))
            (if bSpawnOnEnvironment
              (bind (_outlocation _bhitground) (CallFunction|TraceforGround (.location _output_get)))
              (if _bhitground
                (bind _returnvalue (Components|InstancedStaticMesh|AddInstance (Variables|Default|GetInstancedStaticMesh) (Math|Transform|MakeTransform _outlocation (.rotation (LocalVariables|GetTileTransform)) (.scale (LocalVariables|GetTileTransform))) true))
                (Variables|Default|SetGridLastIndex _returnvalue))
              (else
                (bind _returnvalue_2 (Components|InstancedStaticMesh|AddInstance (Variables|Default|GetInstancedStaticMesh) (LocalVariables|GetTileTransform) true))
                (Variables|Default|SetGridLastIndex _returnvalue_2))))
          (:then_1
            ;[1 1 1] Spawn mesh on uneven collums
            (if (or (!= (LocalVariables|GetXDirection) 0) (!= (LocalVariables|GetYDirection) 0))
              (Utilities|Array|Add (Variables|Default|GetGridLocations) (+ (Variables|Default|GetGridBottomLeftCurrentLocation) (* (Variables|Default|GetGrid%20Tile%20Size) (Math|Vector|MakeVector (- (Math|Conversions|ToFloat(Integer) (LocalVariables|GetXDirection)) 0.5) (/ (* (- (Math|Conversions|ToFloat(Integer) (LocalVariables|GetYDirection)) 0.5) 8.0) 7.0) 0.0))))
              (bind _output_get_2 (LocalVariables|SetTileTransform (Math|Transform|MakeTransform (+ (Variables|Default|GetGridBottomLeftCurrentLocation) (* (Variables|Default|GetGrid%20Tile%20Size) (Math|Vector|MakeVector (- (Math|Conversions|ToFloat(Integer) (LocalVariables|GetXDirection)) 0.5) (/ (* (- (Math|Conversions|ToFloat(Integer) (LocalVariables|GetYDirection)) 0.5) 8.0) 7.0) 0.0))) "0, 0, 0" (/ (Variables|Default|GetGrid%20Tile%20Size) (.MeshSize (CallFunction|GetCurrentShapeData))))))
              (if bSpawnOnEnvironment
                (bind (_outlocation_2 _bhitground_2) (CallFunction|TraceforGround (.location _output_get_2)))
                (if _bhitground_2
                  (bind _returnvalue_3 (Components|InstancedStaticMesh|AddInstance (Variables|Default|GetInstancedStaticMesh) (Math|Transform|MakeTransform _outlocation_2 (.rotation (LocalVariables|GetTileTransform)) (.scale (LocalVariables|GetTileTransform))) true))
                  (Variables|Default|SetGridLastIndex _returnvalue_3))
                (else
                  (bind _returnvalue_4 (Components|InstancedStaticMesh|AddInstance (Variables|Default|GetInstancedStaticMesh) (LocalVariables|GetTileTransform) true))
                  (Variables|Default|SetGridLastIndex _returnvalue_4))))))))))

(fn GetCurrentShapeData
  (bind _returnvalue (Utilities|GetDataTableRow "/Game/Ground/Enum/DT_GridShapeData.DT_GridShapeData" (Utilities|String|StringToName (Utilities|String|EnumtoString (Variables|Default|GetColor))))
    (:then
      (return (.MeshSize (Utilities|Struct|BreakST_GridShapeData _returnvalue)) (.Plane (Utilities|Struct|BreakST_GridShapeData _returnvalue)) (.BorderMaterialInstance (Utilities|Struct|BreakST_GridShapeData _returnvalue)) (Variables|Default|GetGrid%20Tile%20Count)))
    (:RowNotFound
      (Development|PrintString "Error #X9&: Row not found in BP_Grid" true true "(R=1.000000,G=0.000000,B=0.046707,A=1.000000)"))))

(fn SetCurrentShapeData
  (params (Initial%20Spawn%20Location :type Vector) (Tile%20Size :type Vector) (Tile%20Count :type Int%20Point%20Structure) (Color :type E_GridShape%20Enum :default "NewEnumerator0") (Spawn%20Around%20Location :type Boolean) (Spawn%20On%20Environment :type Boolean))
  (Variables|Default|SetInitial%20Spawn%20Location Initial%20Spawn%20Location)
  (Variables|Default|SetGrid%20Tile%20Size Tile%20Size)
  (Variables|Default|SetGrid%20Tile%20Count (Utilities|Struct|MakeIntPoint (.x Tile%20Count) (.y Tile%20Count)))
  (Variables|Default|SetColor Color)
  (Variables|Default|SetbSpawn%20Around%20Given%20Location Spawn%20Around%20Location)
  (Variables|Default|SetbSpawn%20on%20Environment Spawn%20On%20Environment))

(fn DestroyGrid
  (Components|InstancedStaticMesh|ClearInstances (Variables|Default|GetInstancedStaticMesh)))

(fn SnapInitialLocation
  (bind _grid_tile_size (Variables|Default|GetGrid%20Tile%20Size))
  (bind _grid_tile_count (Variables|Default|GetGrid%20Tile%20Count))
  (Variables|Default|SetInitial%20Spawn%20Location (Math|Vector|MakeVector (.x (+ (CallFunction|SnapVectortoVector (Variables|Default|GetInitial%20Spawn%20Location) (Math|Vector|MakeVector (.x _grid_tile_size) (/ (* (.y _grid_tile_size) 8.0) 7.0) (.z _grid_tile_size))) (Math|Vector|MakeVector (+ (LocalVariables|GetXCorrectionFactor1) (/ -1.0 (LocalVariables|GetXCorrectionFactor2))) (LocalVariables|GetYCorrectionFactior) 0.0))) (+ (.y (+ (CallFunction|SnapVectortoVector (Variables|Default|GetInitial%20Spawn%20Location) (Math|Vector|MakeVector (.x _grid_tile_size) (/ (* (.y _grid_tile_size) 8.0) 7.0) (.z _grid_tile_size))) (Math|Vector|MakeVector (+ (LocalVariables|GetXCorrectionFactor1) (/ -1.0 (LocalVariables|GetXCorrectionFactor2))) (LocalVariables|GetYCorrectionFactior) 0.0))) 0.0) (.z (+ (CallFunction|SnapVectortoVector (Variables|Default|GetInitial%20Spawn%20Location) (Math|Vector|MakeVector (.x _grid_tile_size) (/ (* (.y _grid_tile_size) 8.0) 7.0) (.z _grid_tile_size))) (Math|Vector|MakeVector (+ (LocalVariables|GetXCorrectionFactor1) (/ -1.0 (LocalVariables|GetXCorrectionFactor2))) (LocalVariables|GetYCorrectionFactior) 0.0)))))
  (LocalVariables|SetAdjustTileCount (Math|Vector2D|MakeVector2D (Math|Float|SelectFloat 0.0 1.0 (CallFunction|IsIntEven (.x _grid_tile_count))) (Math|Float|SelectFloat 0.0 1.0 (CallFunction|IsIntEven (.y _grid_tile_count)))))
  (if (Variables|Default|GetbSpawn%20Around%20Given%20Location)
    (LocalVariables|SetBottomLeft (Utilities|Operators|Subtract (Variables|Default|GetInitial%20Spawn%20Location) (* (/ (- (Variables|Default|GetGrid%20Tile%20Count) (LocalVariables|GetAdjustTileCount)) "(X=2.000000,Y=2.000000)") (Variables|Default|GetGrid%20Tile%20Size)) (LocalVariables|GetCorrectionFactorOnCentered)))
    (else
      (LocalVariables|SetBottomLeft (- (Variables|Default|GetInitial%20Spawn%20Location) (LocalVariables|GetAdjustTileCount)))))
  (return (LocalVariables|GetBottomLeft)))

(fn SetSpawnAroundGivenLocation
  (params (Spawn%20Around%20Given%20Location :type Boolean))
  (Variables|Default|SetbSpawn%20Around%20Given%20Location Spawn%20Around%20Given%20Location))

(fn GetSpawnAroundGivenLocation
  (return (Variables|Default|GetbSpawn%20Around%20Given%20Location)))

(fn SetGridTileCount
  (params (Grid%20Tile%20Count%20X :type Integer) (Grid%20Tile%20Count%20Y :type Integer))
  (Variables|Default|SetGrid%20Tile%20Count (Utilities|Struct|MakeIntPoint Grid%20Tile%20Count%20X Grid%20Tile%20Count%20Y)))

(fn GetGridTileCount
  (bind _grid_tile_count (Variables|Default|GetGrid%20Tile%20Count))
  (return (.x _grid_tile_count) (.y _grid_tile_count)))

(fn SetGridColor
  (params (Color :type E_GridShape%20Enum :default "NewEnumerator0"))
  (Variables|Default|SetColor Color))

(fn GetGridColor
  (return (Variables|Default|GetColor)))

(fn GetCenterLocation
  (return (/ (+ (.location (.OutInstanceTransform (Components|InstancedStaticMesh|GetInstanceTransform (Variables|Default|GetInstancedStaticMesh) (Variables|Default|GetGridLastIndex) true))) (.location (.OutInstanceTransform (Components|InstancedStaticMesh|GetInstanceTransform (Variables|Default|GetInstancedStaticMesh) 0 true)))) "2.000000,2.000000,2.000000")))

(fn GetBottomLocation
  (bind _gridbottomleftcurrentlocation (Variables|Default|GetGridBottomLeftCurrentLocation))
  (return (+ (Math|Vector|MakeVector (- (.x _gridbottomleftcurrentlocation) (.x (Variables|Default|GetGrid%20Tile%20Size))) (.y _gridbottomleftcurrentlocation) (.z _gridbottomleftcurrentlocation)) (Transformation|GetActorLocation))))

(fn TraceforGround
  (params (Location :type Vector))
  (bind _range (LocalVariables|GetRange))
  (bind _outhits (Collision|MultiSphereTraceByChannel (+ Location _range) (- Location _range) (Variables|Default|GetTraceSphereRadius) "TraceTypeQuery3" false 0 "None"))
  (bind _output_get (LocalVariables|SetHits _outhits))
  (if (> (Utilities|Array|Length _output_get) 0)
    (return (Math|Vector|MakeVector (.x Location) (.y Location) (Math|Float|SnapToGrid(Float) (Utilities|Operators|Subtract (.z (.location (Utilities|Array|Get(acopy) (LocalVariables|GetHits)))) (Variables|Default|GetTraceSphereRadius) -1.0) (.z (Variables|Default|GetGrid%20Tile%20Size)))) true)
    (else
      (return Location false))))