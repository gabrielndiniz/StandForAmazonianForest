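; BP_ActionBase is a base actor for character actions that operate on grid tiles.
; On BeginPlay it finds and caches BP_Grid, retrying on a short delay until valid.
; ExecuteAction returns tile data for two positions and success from the first lookup, or re-fetches the grid and returns failure with placeholder tiles.
; Helpers store the owning pawn and controller, making the controller its owner, and destroy the action.
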(event EventBeginPlay
  (bind _returnvalue (Actor|GetActorOfClass "/Game/Ground/Terrain/BP_Grid.BP_Grid_C" :!label _label))
  (bind _output_get (Variables|Default|SetGrid _returnvalue))
  (Utilities|IsValid _output_get
    (:Is%20Not%20Valid
      (Utilities|FlowControl|Delay 0.2)
      (goto _label))))

(event Collision|EventActorBeginOverlap
  (params (OtherActor :type Actor%20Object%20Reference)))

(fn ConstructionScript)

(fn ExecuteAction
  (params (Position%201 :type Int%20Point%20Structure) (bHitResult :type Boolean) (Position%202 :type Int%20Point%20Structure))
  (bind _array (Utilities|Array|MakeArray "NewEnumerator0"))
  (bind _st_tiledata (Utilities|Struct|MakeST_TileData -1 (Math|Transform|MakeTransform "0, 0, 0" "0, 0, 0" "1.000000,1.000000,1.000000") (Utilities|Struct|MakeIntPoint 999 999) "NewEnumerator0" _array))
  (Utilities|IsValid (Variables|Default|GetGrid)
    (:Is%20Valid
      (return (.Success (Default|GetTileData (Variables|Default|GetGrid) Position%201)) (.TileData (Default|GetTileData (Variables|Default|GetGrid) Position%201)) (.TileData (Default|GetTileData (Variables|Default|GetGrid) Position%202))))
    (:Is%20Not%20Valid
      (bind _returnvalue (Actor|GetActorOfClass "/Game/Ground/Terrain/BP_Grid.BP_Grid_C"))
      (Variables|Default|SetGrid _returnvalue)
      (return false _st_tiledata _st_tiledata))))

(fn DestroyAction
  (Development|PrintString "Being destroyed")
  (Actor|DestroyActor))

(fn SetOwningEntities
  (params (Pawn :type Pawn%20Object%20Reference) (Controller :type Controller%20Object%20Reference))
  (Variables|Components|SetPawn Pawn)
  (bind _output_get (Variables|Default|SetController Controller))
  (Actor|SetOwner _output_get))